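; Roadsign actor that assembles poles, sign boards and mounting hardware in its construction script, taking the board list from the VehicleUI widget's NewSign.
; It uses a single-pole sign mesh from the Style when available, otherwise builds capped poles.
; Mesh sockets position attaches and rails behind each board, with extra builders for rectangles, arrows, text and pictograms.
; Dynamic materials supply sign textures and metal finishes, with randomised dirt offsets on hardware.
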(fn `AddPoles`
  (locals (PolePosition :type "Vector Structure") (PoleHeight :type "Float (double-precision)"))
  (bind (_poleposition_x _poleposition_y _poleposition_z) (`KismetMathLibrary.BreakVector` (`local.PolePosition`)))
  (bind _returnvalue (select `/Game/RoadsignBP/Essentials/Enums/Enum_PoleShape` (`self.Pole Shape`) :`NewEnumerator1` "/Game/RoadsignBP/Essentials/StaticMesh/Pole/SM_roadsign_pole_round_60mm_cap.SM_roadsign_pole_round_60mm_cap" :`NewEnumerator2` "/Game/RoadsignBP/Essentials/StaticMesh/Pole/SM_roadsign_pole_round_76mm_cap.SM_roadsign_pole_round_76mm_cap" :`NewEnumerator3` "/Game/RoadsignBP/Essentials/StaticMesh/Pole/SM_roadsign_pole_square_40x40_cap.SM_roadsign_pole_square_40x40_cap" :`NewEnumerator4` "/Game/RoadsignBP/Essentials/StaticMesh/Pole/SM_roadsign_pole_square_80x80_cap.SM_roadsign_pole_square_80x80_cap" :`NewEnumerator5` "/Game/RoadsignBP/Essentials/StaticMesh/Pole/SM_roadsign_pole_rectangle_40x80_cap.SM_roadsign_pole_rectangle_40x80_cap" :`NewEnumerator6` "/Game/RoadsignBP/Essentials/StaticMesh/Pole/SM_roadsign_pole_H_100mm_cap.SM_roadsign_pole_H_100mm_cap" :!type "StaticMesh Object Reference"))
  (if (select `/Game/RoadsignBP/Essentials/Enums/Enum_PoleShape` (`self.Pole Shape`) :`NewEnumerator1` true :`NewEnumerator2` true :`NewEnumerator3` true :`NewEnumerator4` true :`NewEnumerator5` true :`NewEnumerator6` true)
    (for _array_element (`self.AddPole`)
      (bind (_poleposition _poleheight) (break `/Game/RoadsignBP/Essentials/Structures/S_Roadsigns_AddPole` _array_element))
      (set `local.PolePosition` _poleposition)
      (set `local.PoleHeight` _poleheight)
      (bind _returnvalue_2 (`AddComponent|NODE_AddStaticMeshComponent-1` :`RelativeTransform` (`KismetMathLibrary.MakeTransform` (`KismetMathLibrary.MakeVector` (.x (`local.PolePosition`)) 0.0 (.z (`local.PolePosition`))) (struct) (`KismetMathLibrary.MakeVector` 1.0 1.0 (`local.PoleHeight`))))) ; pole
      (`StaticMeshComponent.SetStaticMesh` _returnvalue_2 (select `/Game/RoadsignBP/Essentials/Enums/Enum_PoleShape` (`self.Pole Shape`) :`NewEnumerator1` "/Game/RoadsignBP/Essentials/StaticMesh/Pole/SM_roadsign_pole_round_60mm.SM_roadsign_pole_round_60mm" :`NewEnumerator2` "/Game/RoadsignBP/Essentials/StaticMesh/Pole/SM_roadsign_pole_round_76mm.SM_roadsign_pole_round_76mm" :`NewEnumerator3` "/Game/RoadsignBP/Essentials/StaticMesh/Pole/SM_roadsign_pole_square_40x40.SM_roadsign_pole_square_40x40" :`NewEnumerator4` "/Game/RoadsignBP/Essentials/StaticMesh/Pole/SM_roadsign_pole_square_80x80.SM_roadsign_pole_square_80x80" :`NewEnumerator5` "/Game/RoadsignBP/Essentials/StaticMesh/Pole/SM_roadsign_pole_rectangle_40x80.SM_roadsign_pole_rectangle_40x80" :`NewEnumerator6` "/Game/RoadsignBP/Essentials/StaticMesh/Pole/SM_roadsign_pole_H_100mm.SM_roadsign_pole_H_100mm" :!type "StaticMesh Object Reference"))
      (bind _material (`self.CreateDynamicMetalMaterial` (`self.PoleMaterial`)))
      (`MaterialInstanceDynamic.SetScalarParameterValue` _material "DirtMap Offset" (`KismetMathLibrary.RandomFloat`))
      (`PrimitiveComponent.SetMaterial` _returnvalue_2 0 _material)
      (bind _returnvalue_3 (`AddComponent|NODE_AddStaticMeshComponent-2` :`RelativeTransform` (`KismetMathLibrary.MakeTransform` (+ (`KismetMathLibrary.MakeVector` (.x (`local.PolePosition`)) 0.0 (.z (`local.PolePosition`))) (`KismetMathLibrary.MakeVector` 0.0 0.0 (`local.PoleHeight`)))))) ; pole cap
      (`StaticMeshComponent.SetStaticMesh` _returnvalue_3 _returnvalue)
      (if (> _poleposition_z 0.0)
        (bind _returnvalue_4 (`AddComponent|NODE_AddStaticMeshComponent-3` :`RelativeTransform` (`KismetMathLibrary.MakeTransform` (`local.PolePosition`) (struct :`Pitch` 180.0)))) ; pole cap
        (`StaticMeshComponent.SetStaticMesh` _returnvalue_4 _returnvalue)))))

(fn `AddSigns`
  (params (hasSinglePole :type Boolean))
  (locals (SignShape :type "/Game/RoadsignBP/Essentials/Enums/Enum_Roadsigns_SignShape Enum") (SignTexture :type "Texture2D Object Reference") (SignTransform :type "Transform Structure") (SignYLocation :type "Float (double-precision)") (NULLParent :type "SceneComponent Object Reference") (SignMesh :type "StaticMesh Object Reference") (SignMetalMaterialInstance :type "MaterialInstanceDynamic Object Reference") (signMaterial :type "MaterialInstanceDynamic Object Reference") (isIridescent :type Boolean) (AttachMesh :type "StaticMesh Object Reference") (PoleLocationX :type "Float (double-precision)" :default 0.0) (RailIndex :type Integer) (SignMeshComponent :type "StaticMeshComponent Object Reference") (AttachMeshComponent :type "StaticMeshComponent Object Reference") (RailMeshComponent :type "StaticMeshComponent Object Reference") (DefaultAttachCOmponent :type "SceneComponent Object Reference") (TextElements :type "Array of /Game/RoadsignBP/Essentials/Structures/S_Roadsigns_TextParameters Structure") (PictoElements :type "Array of /Game/RoadsignBP/Essentials/Structures/S_Roadsigns_Picto Structure"))
  (bind _addsignboard (`self.AddSignBoard`))
  (bind _signmeshcomponent (`local.SignMeshComponent`))
  (bind _railmeshcomponent (`local.RailMeshComponent`))
  (bind _signtransform (`local.SignTransform`))
  (bind _signtransform_2 (`local.SignTransform`))
  (bind _signtransform_3 (`local.SignTransform`))
  (bind _signtransform_4 (`local.SignTransform`))
  (bind _signtransform_5 (`local.SignTransform`))
  (bind _style (`self.Style`))
  (bind _style_2 (`self.Style`))
  (bind _style_3 (`self.Style`))
  (bind (_min _max) (`StaticMeshComponent.GetLocalBounds` _signmeshcomponent))
  (bind (_relativelocation_x _relativelocation_y _relativelocation_z) (`KismetMathLibrary.BreakVector` (`SceneComponent.RelativeLocation` (`local.AttachMeshComponent`))))
  (bind (_relativelocation_x_2 _relativelocation_y_2 _relativelocation_z_2) (`KismetMathLibrary.BreakVector` (`SceneComponent.RelativeLocation` (`local.AttachMeshComponent`))))
  (bind (_relativelocation_x_3 _relativelocation_y_3 _relativelocation_z_3) (`KismetMathLibrary.BreakVector` (`SceneComponent.RelativeLocation` (`local.NULLParent`))))
  (bind _relativelocation_x_4 (`KismetMathLibrary.BreakVector` (`SceneComponent.RelativeLocation` _signmeshcomponent)))
  (bind _railmesh (`/Game/RoadsignBP/Essentials/BP/BP_DA_Roadsign_Style.RailMesh` (`self.Style`)))
  (bind _returnvalue (`StaticMesh.FindSocket` _railmesh "sign"))
  (bind _returnvalue_2 (- (.x _max) (.x _min)))
  (bind (_relativelocation_x_5 _relativelocation_y_4) (`KismetMathLibrary.BreakVector` (`StaticMeshSocket.RelativeLocation` (`StaticMesh.FindSocket` (`local.AttachMesh`) "rail"))))
  (bind (_relativelocation_x_6 _relativelocation_y_5) (`KismetMathLibrary.BreakVector` (`StaticMeshSocket.RelativeLocation` (`StaticMesh.FindSocket` (`local.AttachMesh`) "rail"))))
  (bind (_relativelocation_x_7 _relativelocation_y_6) (`KismetMathLibrary.BreakVector` (`StaticMeshSocket.RelativeLocation` (`StaticMesh.FindSocket` (`/Game/RoadsignBP/Essentials/BP/BP_DA_Roadsign_Style.RailMesh` (`self.Style`)) "attach"))))
  (bind (_relativelocation_x_8 _relativelocation_y_7) (`KismetMathLibrary.BreakVector` (`StaticMeshSocket.RelativeLocation` (`StaticMesh.FindSocket` _railmesh "attach"))))
  (bind (_relativelocation_x_9 _relativelocation_y_8) (`KismetMathLibrary.BreakVector` (`StaticMeshSocket.RelativeLocation` _returnvalue)))
  (bind (_relativelocation_x_10 _relativelocation_y_9) (`KismetMathLibrary.BreakVector` (`StaticMeshSocket.RelativeLocation` (`StaticMesh.FindSocket` (`/Game/RoadsignBP/Essentials/BP/BP_DA_Roadsign_Style.RailMesh` (`self.Style`)) "attach"))))
  (bind (_relativelocation_x_11 _relativelocation_y_10) (`KismetMathLibrary.BreakVector` (`StaticMeshSocket.RelativeLocation` (`StaticMesh.FindSocket` (select `/Game/RoadsignBP/Essentials/Enums/Enum_PoleShape` (`self.Pole Shape`) :`NewEnumerator1` (`/Game/RoadsignBP/Essentials/BP/BP_DA_Roadsign_Style.Attach Circle Ø60mm` _style_3) :`NewEnumerator2` (`/Game/RoadsignBP/Essentials/BP/BP_DA_Roadsign_Style.Attach Circle Ø76mm` _style_3) :`NewEnumerator3` (`/Game/RoadsignBP/Essentials/BP/BP_DA_Roadsign_Style.Attach Square 40mm` _style_3) :`NewEnumerator4` (`/Game/RoadsignBP/Essentials/BP/BP_DA_Roadsign_Style.Attach Square 80mm` _style_3) :`NewEnumerator5` (`/Game/RoadsignBP/Essentials/BP/BP_DA_Roadsign_Style.Attach Rectangle 40x 80mm` _style_3) :`NewEnumerator6` (`/Game/RoadsignBP/Essentials/BP/BP_DA_Roadsign_Style.Attach H 100mm` _style_3)) "rail"))))
  (bind (_relativelocation_x_12 _relativelocation_y_11 _relativelocation_z_4) (`KismetMathLibrary.BreakVector` (`StaticMeshSocket.RelativeLocation` (`StaticMesh.FindSocket` (`local.SignMesh`) (`KismetStringLibrary.Conv_StringToName` (`KismetStringLibrary.Concat_StrStr` "rail" (`KismetStringLibrary.Conv_IntToString` (`local.RailIndex`))))))))
  (bind (_relativelocation_x_13 _relativelocation_y_12 _relativelocation_z_5) (`KismetMathLibrary.BreakVector` (`StaticMeshSocket.RelativeLocation` (`StaticMesh.FindSocket` (`local.SignMesh`) (`KismetStringLibrary.Conv_StringToName` (`KismetStringLibrary.Concat_StrStr` "rail" (`KismetStringLibrary.Conv_IntToString` (`local.RailIndex`))))))))
  (if (`KismetArrayLibrary.Array_IsNotEmpty` _addsignboard)
    (for (_array_element _array_index) _addsignboard
      (if (not (and (== _array_index 0) (`local.hasSinglePole`)))
        (bind (_signshape _signtexture _iridescent _transform _addtextelement _addpictoelement) (break `/Game/RoadsignBP/Essentials/Structures/S_Roadsigns_AddSign` _array_element))
        (set `local.SignShape` _signshape)
        (set `local.SignTexture` _signtexture)
        (set `local.isIridescent` _iridescent)
        (set `local.SignTransform` _transform)
        (set `local.TextElements` _addtextelement)
        (set `local.PictoElements` _addpictoelement)
        (`KismetArrayLibrary.Array_Set` (`self.AddSignBoard`) _array_index (make `/Game/RoadsignBP/Essentials/Structures/S_Roadsigns_AddSign` (`local.SignShape`) (`local.SignTexture`) (`local.isIridescent`) (`KismetMathLibrary.MakeTransform` (`KismetMathLibrary.MakeVector` (.x (.location _signtransform_2)) (.y (.location _signtransform_2)) (.z (.location _signtransform_2))) (`KismetMathLibrary.MakeRotator` 0.0 0.0 (.yaw (.rotation _signtransform_2))) (`KismetMathLibrary.MakeVector` (.x (.scale _signtransform_2)) 1.0 (.z (.scale _signtransform_2)))) (`local.TextElements`) (`local.PictoElements`)))
        (set `local.SignMesh` (select `/Game/RoadsignBP/Essentials/Enums/Enum_Roadsigns_SignShape` (`local.SignShape`) :`NewEnumerator0` (`/Game/RoadsignBP/Essentials/BP/BP_DA_Roadsign_Style.RoundSignMesh` _style) :`NewEnumerator1` (`/Game/RoadsignBP/Essentials/BP/BP_DA_Roadsign_Style.TriangleSignMesh` _style) :`NewEnumerator2` (`/Game/RoadsignBP/Essentials/BP/BP_DA_Roadsign_Style.SquareSignMesh` _style) :`NewEnumerator3` (`/Game/RoadsignBP/Essentials/BP/BP_DA_Roadsign_Style.DiamondSignMesh` _style) :`NewEnumerator4` (`/Game/RoadsignBP/Essentials/BP/BP_DA_Roadsign_Style.StopSignMesh` _style) :`NewEnumerator5` (`/Game/RoadsignBP/Essentials/BP/BP_DA_Roadsign_Style.Panel` _style) :`NewEnumerator6` (`/Game/RoadsignBP/Essentials/BP/BP_DA_Roadsign_Style.ArrowCenter_1Lign` _style) :`NewEnumerator7` (`/Game/RoadsignBP/Essentials/BP/BP_DA_Roadsign_Style.ArrowCenter_2Ligns` _style) :`NewEnumerator8` (`/Game/RoadsignBP/Essentials/BP/BP_DA_Roadsign_Style.ArrowCenter_3Ligns` _style)))
        ;[1 1 1] reset components
        (set `local.AttachMeshComponent` null)
        (set `local.RailMeshComponent` null)
        (set `local.AttachMesh` (select `/Game/RoadsignBP/Essentials/Enums/Enum_PoleShape` (`self.Pole Shape`) :`NewEnumerator1` (`/Game/RoadsignBP/Essentials/BP/BP_DA_Roadsign_Style.Attach Circle Ø60mm` _style_2) :`NewEnumerator2` (`/Game/RoadsignBP/Essentials/BP/BP_DA_Roadsign_Style.Attach Circle Ø76mm` _style_2) :`NewEnumerator3` (`/Game/RoadsignBP/Essentials/BP/BP_DA_Roadsign_Style.Attach Square 40mm` _style_2) :`NewEnumerator4` (`/Game/RoadsignBP/Essentials/BP/BP_DA_Roadsign_Style.Attach Square 80mm` _style_2) :`NewEnumerator5` (`/Game/RoadsignBP/Essentials/BP/BP_DA_Roadsign_Style.Attach Rectangle 40x 80mm` _style_2) :`NewEnumerator6` (`/Game/RoadsignBP/Essentials/BP/BP_DA_Roadsign_Style.Attach H 100mm` _style_2)))
        (`/Engine/EditorBlueprintResources/StandardMacros.IsValid` _returnvalue
          (:`Is Valid`
            (set `local.SignYLocation` (- _relativelocation_y_4 _relativelocation_y_7 _relativelocation_y_8)))
          (:`Is Not Valid`
            (set `local.SignYLocation` (- _relativelocation_y_5 _relativelocation_y_9 0.0))))
        (bind _returnvalue_3 (`AddComponent|NODE_AddSceneComponent-0` :`RelativeTransform` (`KismetMathLibrary.MakeTransform` (`KismetMathLibrary.MakeVector` 0.0 0.0 (.z (.location (`local.SignTransform`)))) (`KismetMathLibrary.MakeRotator` 0.0) (1.0 1.0 1.0))))
        (set `local.NULLParent` _returnvalue_3)
        (`|ExecutionSequence`
          (:`then_0`
            ;[0.1551 0.2604 0.1524] RoadSign
            (bind _returnvalue_4 (`AddComponent|NODE_AddStaticMeshComponent-6` :`RelativeTransform` (`KismetMathLibrary.MakeTransform` (`KismetMathLibrary.MakeVector` (.x (.location _signtransform_3)) (`local.SignYLocation`)) (`KismetMathLibrary.MakeRotator` 0.0) (`KismetMathLibrary.MakeVector` (.x (.scale _signtransform_3)) 1.0 (.z (.scale _signtransform_3))))))
            (set `local.SignMeshComponent` _returnvalue_4)
            (`SceneComponent.K2_AttachToComponent` (`local.SignMeshComponent`) (`local.NULLParent`) "None" "KeepRelative" "KeepRelative" "KeepWorld" true)
            (`StaticMeshComponent.SetStaticMesh` (`local.SignMeshComponent`) (`local.SignMesh`))
            (bind _material (`self.CreateDynamicMetalMaterial` (`self.SignMetalMaterial`) (`local.SignMesh`)))
            (set `local.SignMetalMaterialInstance` _material)
            (`PrimitiveComponent.SetMaterialByName` (`local.SignMeshComponent`) "metal" _material)
            (bind _material_2 (`self.CreateDynamicSignMaterial` (`local.SignTexture`) (`local.isIridescent`) (`local.SignMesh`)))
            (bind _output_get (set `local.signMaterial` _material_2))
            (`PrimitiveComponent.SetMaterialByName` (`local.SignMeshComponent`) "sign" _output_get))
          (:`then_1`
            ;[0.08854 0.08854 0.08854] Attaches
            (for _index (range 1 5)
              (set `local.RailIndex` _index)
              (`/Engine/EditorBlueprintResources/StandardMacros.IsValid` (`StaticMesh.FindSocket` (`local.SignMesh`) (`KismetStringLibrary.Conv_StringToName` (`KismetStringLibrary.Concat_StrStr` "rail" (`KismetStringLibrary.Conv_IntToString` (`local.RailIndex`)))))
                (:`Is Valid`
                  (if (and (`|EnumInequality` (`self.Pole Shape`) "NewEnumerator0") (`KismetArrayLibrary.Array_IsNotEmpty` (`self.AddPole`)))
                    (for _array_element_2 (`self.AddPole`)
                      (bind (_poleposition _poleheight) (break `/Game/RoadsignBP/Essentials/Structures/S_Roadsigns_AddPole` _array_element_2))
                      (bind _output_get_2 (set `local.PoleLocationX` (.x _poleposition)))
                      (if (and (> (+ _output_get_2 20.0) (+ (* _returnvalue_2 -1.0) _relativelocation_x_4)) (< (- _output_get_2 20.0) (+ _returnvalue_2 _relativelocation_x_4)) (> (+ (.z _poleposition) _poleheight) _relativelocation_z_3) (< (.z _poleposition) _relativelocation_z_3))
                        (bind _returnvalue_5 (`AddComponent|NODE_AddStaticMeshComponent-4` :`RelativeTransform` (`KismetMathLibrary.MakeTransform` (`KismetMathLibrary.MakeVector` (`local.PoleLocationX`) 0.0 (+ (* (.z (.scale (`local.SignTransform`))) _relativelocation_z_5) (.z (.location _signtransform_5)))) (`KismetMathLibrary.MakeRotator` 0.0 0.0 (.yaw (.rotation _signtransform_5))))))
                        (set `local.AttachMeshComponent` _returnvalue_5)
                        (`SceneComponent.K2_AttachToComponent` (`local.AttachMeshComponent`) (`local.NULLParent`) "None" "KeepWorld" "KeepRelative" "KeepWorld" true :!label _label)
                        (bind _material_3 (`self.CreateDynamicMetalMaterial` (`self.AttachMaterial`) (`local.AttachMesh`)))
                        (`MaterialInstanceDynamic.SetScalarParameterValue` _material_3 "DirtMap Offset" (`KismetMathLibrary.RandomFloat`))
                        (`PrimitiveComponent.SetMaterial` (`local.AttachMeshComponent`) 0 _material_3)
                        (`StaticMeshComponent.SetStaticMesh` (`local.AttachMeshComponent`) (`local.AttachMesh`))))
                    (else
                      (bind _returnvalue_6 (`AddComponent|NODE_AddStaticMeshComponent-7` :`RelativeTransform` (`KismetMathLibrary.MakeTransform` (`KismetMathLibrary.MakeVector` (.x (.location _signtransform)) 0.0 (+ (* (.z (.scale _signtransform)) _relativelocation_z_4) (.z (.location _signtransform_4)))) (`KismetMathLibrary.MakeRotator` 0.0 0.0 (.yaw (.rotation _signtransform_4))))))
                      (set `local.AttachMeshComponent` _returnvalue_6)
                      (goto _label))))
                (:`Is Not Valid`
                  (break)))))
          (:`then_2`
            ;[1 1 1] Rail
            (`local.AttachMeshComponent`
              (:`then`
                (for _index_2 (range 1 5)
                  (bind _returnvalue_7 (`StaticMesh.FindSocket` (`local.SignMesh`) (`KismetStringLibrary.Conv_StringToName` (`KismetStringLibrary.Concat_StrStr` "rail" (`KismetStringLibrary.Conv_IntToString` _index_2)))))
                  (`/Engine/EditorBlueprintResources/StandardMacros.IsValid` _returnvalue_7
                    (:`Is Valid`
                      (bind (_relativelocation_x_14 _relativelocation_y_13 _relativelocation_z_6) (`KismetMathLibrary.BreakVector` (`StaticMeshSocket.RelativeLocation` _returnvalue_7)))
                      (bind _relativescale_x (`KismetMathLibrary.BreakVector` (`StaticMeshSocket.RelativeScale` _returnvalue_7)))
                      (bind _returnvalue_8 (`AddComponent|NODE_AddStaticMeshComponent-5` :`RelativeTransform` (`KismetMathLibrary.MakeTransform` (`KismetMathLibrary.MakeVector` (- (.x (.location (`local.SignTransform`))) _relativelocation_x_2) (- _relativelocation_y_10 _relativelocation_y_6) (- (* (.z (.scale (`local.SignTransform`))) _relativelocation_z_6) _relativelocation_z_2)) (`KismetMathLibrary.MakeRotator` 0.0) (`KismetMathLibrary.MakeVector` (* _relativescale_x (.x (.scale (`local.SignTransform`)))) 1.0 1.0))))
                      (set `local.RailMeshComponent` _returnvalue_8)
                      (`SceneComponent.K2_AttachToComponent` _returnvalue_8 (`local.AttachMeshComponent`) "None" "KeepRelative" "KeepRelative" "KeepWorld" true)
                      (`StaticMeshComponent.SetStaticMesh` _returnvalue_8 (`/Game/RoadsignBP/Essentials/BP/BP_DA_Roadsign_Style.RailMesh` (`self.Style`)))
                      (bind _material_4 (`self.CreateDynamicMetalMaterial` (`self.SignMetalMaterial`) (`/Game/RoadsignBP/Essentials/BP/BP_DA_Roadsign_Style.RailMesh` (`self.Style`))))
                      (`MaterialInstanceDynamic.SetScalarParameterValue` _material_4 "DirtMap Offset" (`KismetMathLibrary.RandomFloat`))
                      (`PrimitiveComponent.SetMaterial` _returnvalue_8 0 _material_4))
                    (:`Is Not Valid`
                      (break)))))
              (:`else`)))
          (:`then_3`
            ;[0.1775 0.1372 0.1979] Custom Rectangle
            (if (`|EnumEquality` (`local.SignShape`) "NewEnumerator5")
              (`MaterialInstanceDynamic.SetScalarParameterValue` (`local.SignMetalMaterialInstance`) "UseCornerMask" (`KismetMathLibrary.Conv_BoolToDouble` (`/Game/RoadsignBP/Essentials/BP/BP_DA_Roadsign_Style.isRoundCorner` (`self.Style`))))
              (`MaterialInstanceDynamic.SetScalarParameterValue` (`local.signMaterial`) "UseCornerMask" (`KismetMathLibrary.Conv_BoolToDouble` (`/Game/RoadsignBP/Essentials/BP/BP_DA_Roadsign_Style.isRoundCorner` (`self.Style`))))
              (`self.CreateCustomRectangle` (`local.SignMeshComponent`) (`local.SignMetalMaterialInstance`) (`local.signMaterial`) (`local.SignTransform`) (`self.Style`))))
          (:`then_4`
            (if (select `/Game/RoadsignBP/Essentials/Enums/Enum_Roadsigns_SignShape` (`local.SignShape`) :`NewEnumerator6` true :`NewEnumerator7` true :`NewEnumerator8` true)
              (`self.CreateArrow` (`local.SignMeshComponent`) (`local.SignMetalMaterialInstance`) (`local.signMaterial`) (`local.SignTransform`) (`local.SignShape`) (`self.Style`))))
          (:`then_5`
            (`local.RailMeshComponent`
              (:`then`
                _)
              (:`else`
                (`KismetSystemLibrary.PrintString` (`KismetStringLibrary.Concat_StrStr` (`KismetSystemLibrary.GetDisplayName` self) " : Bad Roadsign Position") true true (struct :`R` 1.0 :`A` 1.0))))
            (`SceneComponent.K2_AttachToComponent` (`local.SignMeshComponent`) (select `bool` (`KismetSystemLibrary.IsValid` _railmeshcomponent) :`true` _railmeshcomponent :!type "SceneComponent Object Reference") "None" "KeepRelative" "KeepRelative" "KeepWorld" true)
            (`SceneComponent.K2_SetRelativeLocation` (`local.SignMeshComponent`) (`KismetMathLibrary.MakeVector` 0.0 0.0 (* _relativelocation_z -1.0)) false false))
          (:`then_6`
            (for _array_element_3 (`local.TextElements`)
              (`self.AddTextElement` _array_element_3 (`local.SignMeshComponent`) (`local.isIridescent`) (`local.SignTransform`) (`self.Text Font`))))
          (:`then_7`
            (for _array_element_4 (`local.PictoElements`)
              (`self.AddPictoElement` _array_element_4 (`local.SignMeshComponent`) (`local.isIridescent`) (`local.SignTransform`)))))))))

(fn `ChangeSignMaterial`
  (params (NewMaterial :type "MaterialInstanceDynamic Object Reference"))
  (return))

(fn `CreateSinglePoleSign`
  (returns (isSuccess :type Boolean))
  (locals (success :type Boolean) (SinglePoleStaticMesh :type "StaticMesh Object Reference" :default "/Script/Engine.StaticMesh'/Game/RoadsignBP/Essentials/StaticMesh/Pole/SM_roadsign_pole_round_60mm.SM_roadsign_pole_round_60mm'"))
  (bind _style (`self.Style`))
  (bind _output_poleposition (break `/Game/RoadsignBP/Essentials/Structures/S_Roadsigns_AddPole` (`|GetArrayItem` (`self.AddPole`))))
  (bind (_output_signshape _output_signtexture _output_iridescent) (break `/Game/RoadsignBP/Essentials/Structures/S_Roadsigns_AddSign` (`|GetArrayItem` (`self.AddSignBoard`))))
  (bind _output_signshape_2 (break `/Game/RoadsignBP/Essentials/Structures/S_Roadsigns_AddSign` (`|GetArrayItem` (`self.AddSignBoard`))))
  (bind _returnvalue (select `/Game/RoadsignBP/Essentials/Enums/Enum_Roadsigns_SignShape` _output_signshape_2 :`NewEnumerator0` (`/Game/RoadsignBP/Essentials/BP/BP_DA_Roadsign_Style.SingleRoundSignMesh` _style) :`NewEnumerator1` (`/Game/RoadsignBP/Essentials/BP/BP_DA_Roadsign_Style.SingleTriangleSignMesh` _style) :`NewEnumerator2` (`/Game/RoadsignBP/Essentials/BP/BP_DA_Roadsign_Style.SingleSquareSignMesh` _style) :`NewEnumerator3` (`/Game/RoadsignBP/Essentials/BP/BP_DA_Roadsign_Style.SingleDiamondSignMesh` _style) :`NewEnumerator4` (`/Game/RoadsignBP/Essentials/BP/BP_DA_Roadsign_Style.SingleStopSignMesh` _style)))
  (`|ExecutionSequence`
    (:`then_0`
      (if (and (`self.useSinglePoleSignDefinitionIfAvailable`) (== (`KismetArrayLibrary.Array_Length` (`self.AddPole`)) 1))
        (`/Engine/EditorBlueprintResources/StandardMacros.IsValid` _returnvalue
          (:`Is Valid`
            (set `local.SinglePoleStaticMesh` _returnvalue)
            (bind _returnvalue_2 (`AddComponent|NODE_AddStaticMeshComponent-0` :`RelativeTransform` (`KismetMathLibrary.MakeTransform` _output_poleposition (struct) (1.0 1.0 1.0)))) ; pole
            (bind _returnvalue_3 (`StaticMeshComponent.SetStaticMesh` _returnvalue_2 (`local.SinglePoleStaticMesh`)))
            (set `local.success` _returnvalue_3)
            (bind _material (`self.CreateDynamicMetalMaterial` (`self.PoleMaterial`)))
            (`PrimitiveComponent.SetMaterialByName` _returnvalue_2 "metal" _material)
            (`MaterialInstanceDynamic.SetTextureParameterValue` _material "Normal" (`self.GetNormalFromMesh` (`local.SinglePoleStaticMesh`)))
            (bind _material_2 (`self.CreateDynamicSignMaterial` _output_signtexture _output_iridescent (`local.SinglePoleStaticMesh`)))
            (`PrimitiveComponent.SetMaterialByName` _returnvalue_2 "sign" _material_2))
          (:`Is Not Valid`
            (set `local.success` false)))
        (else
          (set `local.success` false))))
    (:`then_1`
      (return (`local.success`)))))

(fn `SetBillboard`
  (bind _billboard (`self.Billboard`))
  (if (and (`KismetArrayLibrary.Array_IsEmpty` (`self.AddPole`)) (`KismetArrayLibrary.Array_IsEmpty` (`self.AddSignBoard`)))
    (`SceneComponent.SetVisibility` _billboard true false)
    (else
      (`SceneComponent.SetVisibility` _billboard false false))))

(fn `UserConstructionScript`
  (`parent.UserConstructionScript`)
  (bind _foundwidgets (`WidgetBlueprintLibrary.GetAllWidgetsOfClass` "/Game/VehicleTemplate/Blueprints/VehicleUI.VehicleUI_C"))
  (set `self.AddSignBoard` (`/Game/VehicleTemplate/Blueprints/VehicleUI.NewSign` (`|GetArrayItem` _foundwidgets)))
  (`self.SetBillboard`)
  (bind _issuccess (`self.CreateSinglePoleSign`))
  (if (not _issuccess)
    (`self.AddPoles`))
  (`self.AddSigns` _issuccess))