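; Road sign board actor that assembles a single sign in the construction script from a Style and Roadsign settings.
; It snaps to an optional parent actor, taking the pole shape from a BP_Roadsign_1Pole to choose the bracket mesh.
; Numbered "rail" sockets on the sign mesh position brackets and rails.
; Dynamic materials randomise dirt offsets, with helpers for custom rectangles, arrows, text and pictograms.
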(fn `CreateRoadsign`
  (locals (SignShape :type "/Game/RoadsignBP/Essentials/Enums/Enum_Roadsigns_SignShape Enum") (SignTexture :type "Texture2D Object Reference") (isIridescent :type Boolean) (SignTransform :type "Transform Structure") (SignMesh :type "StaticMesh Object Reference") (AttachMesh :type "StaticMesh Object Reference") (SignYLocation :type "Float (double-precision)") (NULLParent :type "SceneComponent Object Reference") (SignMeshComponent :type "StaticMeshComponent Object Reference") (signMaterial :type "MaterialInstanceDynamic Object Reference") (RailIndex :type Integer) (PoleLocationX :type "Float (double-precision)") (AttachMeshComponent :type "StaticMeshComponent Object Reference") (RailMeshComponent :type "StaticMeshComponent Object Reference") (SignMetalMaterialInstance :type "MaterialInstanceDynamic Object Reference") (TextElements :type "Array of /Game/RoadsignBP/Essentials/Structures/S_Roadsigns_TextParameters Structure") (PictoElements :type "Array of /Game/RoadsignBP/Essentials/Structures/S_Roadsigns_Picto Structure"))
  (bind _style (`self.Style`))
  (bind _signtransform (`local.SignTransform`))
  (bind _roadsign_signshape (break `/Game/RoadsignBP/Essentials/Structures/S_Roadsigns_AddSign` (`self.Roadsign`)))
  (bind (_roadsign_signshape_2 _roadsign_signtexture _roadsign_iridescent _roadsign_transform _roadsign_addtextelement _roadsign_addpictoelement) (break `/Game/RoadsignBP/Essentials/Structures/S_Roadsigns_AddSign` (`self.Roadsign`)))
  (bind _railmeshcomponent (`local.RailMeshComponent`))
  (bind _signtransform_2 (`local.SignTransform`))
  (bind (_roadsign_signshape_3 _roadsign_signtexture_2 _roadsign_iridescent_2 _roadsign_transform_2 _roadsign_addtextelement_2 _roadsign_addpictoelement_2) (break `/Game/RoadsignBP/Essentials/Structures/S_Roadsigns_AddSign` (`self.Roadsign`)))
  (bind _signtransform_3 (`local.SignTransform`))
  (bind _style_2 (`self.Style`))
  (bind _style_3 (`self.Style`))
  (bind _scale (.scale _roadsign_transform))
  (bind _returnvalue (`StaticMesh.GetBoundingBox` (`local.SignMesh`)))
  (bind (_relativelocation_x _relativelocation_y _relativelocation_z) (`KismetMathLibrary.BreakVector` (`SceneComponent.RelativeLocation` (`local.AttachMeshComponent`))))
  (bind (_relativelocation_x_2 _relativelocation_y_2 _relativelocation_z_2) (`KismetMathLibrary.BreakVector` (`SceneComponent.RelativeLocation` (`local.AttachMeshComponent`))))
  (bind _railmesh (`/Game/RoadsignBP/Essentials/BP/BP_DA_Roadsign_Style.RailMesh` (`self.Style`)))
  (bind _x (.x _scale))
  (bind (_relativelocation_x_3 _relativelocation_y_3) (`KismetMathLibrary.BreakVector` (`StaticMeshSocket.RelativeLocation` (`StaticMesh.FindSocket` (`local.AttachMesh`) "rail"))))
  (bind (_relativelocation_x_4 _relativelocation_y_4) (`KismetMathLibrary.BreakVector` (`StaticMeshSocket.RelativeLocation` (`StaticMesh.FindSocket` (`/Game/RoadsignBP/Essentials/BP/BP_DA_Roadsign_Style.RailMesh` (`self.Style`)) "attach"))))
  (bind (_relativelocation_x_5 _relativelocation_y_5) (`KismetMathLibrary.BreakVector` (`StaticMeshSocket.RelativeLocation` (`StaticMesh.FindSocket` _railmesh "attach"))))
  (bind (_relativelocation_x_6 _relativelocation_y_6) (`KismetMathLibrary.BreakVector` (`StaticMeshSocket.RelativeLocation` (`StaticMesh.FindSocket` _railmesh "sign"))))
  (bind (_relativelocation_x_7 _relativelocation_y_7) (`KismetMathLibrary.BreakVector` (`StaticMeshSocket.RelativeLocation` (`StaticMesh.FindSocket` (select `/Game/RoadsignBP/Essentials/Enums/Enum_PoleShape` (`self.Pole Shape`) :`NewEnumerator1` (`/Game/RoadsignBP/Essentials/BP/BP_DA_Roadsign_Style.Attach Circle Ø60mm` _style_3) :`NewEnumerator2` (`/Game/RoadsignBP/Essentials/BP/BP_DA_Roadsign_Style.Attach Circle Ø76mm` _style_3) :`NewEnumerator3` (`/Game/RoadsignBP/Essentials/BP/BP_DA_Roadsign_Style.Attach Square 40mm` _style_3) :`NewEnumerator4` (`/Game/RoadsignBP/Essentials/BP/BP_DA_Roadsign_Style.Attach Square 80mm` _style_3) :`NewEnumerator5` (`/Game/RoadsignBP/Essentials/BP/BP_DA_Roadsign_Style.Attach Rectangle 40x 80mm` _style_3) :`NewEnumerator6` (`/Game/RoadsignBP/Essentials/BP/BP_DA_Roadsign_Style.Attach H 100mm` _style_3)) "rail"))))
  (bind (_relativelocation_x_8 _relativelocation_y_8 _relativelocation_z_3) (`KismetMathLibrary.BreakVector` (`StaticMeshSocket.RelativeLocation` (`StaticMesh.FindSocket` (`local.SignMesh`) (`KismetStringLibrary.Conv_StringToName` (`KismetStringLibrary.Concat_StrStr` "rail" (`KismetStringLibrary.Conv_IntToString` (`local.RailIndex`))))))))
  (set `local.SignMesh` (select `/Game/RoadsignBP/Essentials/Enums/Enum_Roadsigns_SignShape` _roadsign_signshape :`NewEnumerator0` (`/Game/RoadsignBP/Essentials/BP/BP_DA_Roadsign_Style.RoundSignMesh` _style) :`NewEnumerator1` (`/Game/RoadsignBP/Essentials/BP/BP_DA_Roadsign_Style.TriangleSignMesh` _style) :`NewEnumerator2` (`/Game/RoadsignBP/Essentials/BP/BP_DA_Roadsign_Style.SquareSignMesh` _style) :`NewEnumerator3` (`/Game/RoadsignBP/Essentials/BP/BP_DA_Roadsign_Style.DiamondSignMesh` _style) :`NewEnumerator4` (`/Game/RoadsignBP/Essentials/BP/BP_DA_Roadsign_Style.StopSignMesh` _style) :`NewEnumerator5` (`/Game/RoadsignBP/Essentials/BP/BP_DA_Roadsign_Style.Panel` _style) :`NewEnumerator6` (`/Game/RoadsignBP/Essentials/BP/BP_DA_Roadsign_Style.ArrowCenter_1Lign` _style) :`NewEnumerator7` (`/Game/RoadsignBP/Essentials/BP/BP_DA_Roadsign_Style.ArrowCenter_2Ligns` _style) :`NewEnumerator8` (`/Game/RoadsignBP/Essentials/BP/BP_DA_Roadsign_Style.ArrowCenter_3Ligns` _style)))
  (set `self.Roadsign` (make `/Game/RoadsignBP/Essentials/Structures/S_Roadsigns_AddSign` _roadsign_signshape_2 _roadsign_signtexture _roadsign_iridescent (`KismetMathLibrary.MakeTransform` (`KismetMathLibrary.MakeVector` (`KismetMathLibrary.FClamp` (.x (.location _roadsign_transform)) (- (* (.x (break `Box` _returnvalue)) _x) 20.0) (+ (* (.x (`.Max` (break `Box` _returnvalue))) _x) 20.0)) 0.0 (.z (.location _roadsign_transform))) (`KismetMathLibrary.MakeRotator` 0.0 0.0 (.yaw (.rotation _roadsign_transform))) _scale) _roadsign_addtextelement _roadsign_addpictoelement))
  (set `local.SignShape` _roadsign_signshape_3)
  (set `local.SignTexture` _roadsign_signtexture_2)
  (set `local.isIridescent` _roadsign_iridescent_2)
  (set `local.SignTransform` _roadsign_transform_2)
  (set `local.TextElements` _roadsign_addtextelement_2)
  (set `local.PictoElements` _roadsign_addpictoelement_2)
  (set `local.AttachMesh` (select `/Game/RoadsignBP/Essentials/Enums/Enum_PoleShape` (`self.Pole Shape`) :`NewEnumerator1` (`/Game/RoadsignBP/Essentials/BP/BP_DA_Roadsign_Style.Attach Circle Ø60mm` _style_2) :`NewEnumerator2` (`/Game/RoadsignBP/Essentials/BP/BP_DA_Roadsign_Style.Attach Circle Ø76mm` _style_2) :`NewEnumerator3` (`/Game/RoadsignBP/Essentials/BP/BP_DA_Roadsign_Style.Attach Square 40mm` _style_2) :`NewEnumerator4` (`/Game/RoadsignBP/Essentials/BP/BP_DA_Roadsign_Style.Attach Square 80mm` _style_2) :`NewEnumerator5` (`/Game/RoadsignBP/Essentials/BP/BP_DA_Roadsign_Style.Attach Rectangle 40x 80mm` _style_2) :`NewEnumerator6` (`/Game/RoadsignBP/Essentials/BP/BP_DA_Roadsign_Style.Attach H 100mm` _style_2)))
  (set `local.SignYLocation` (- _relativelocation_y_3 _relativelocation_y_5 _relativelocation_y_6))
  (bind _returnvalue_2 (`AddComponent|NODE_AddSceneComponent-0` :`RelativeTransform` (`KismetMathLibrary.MakeTransform` (`KismetMathLibrary.MakeVector` 0.0 0.0 (.z (.location (`local.SignTransform`)))))))
  (set `local.NULLParent` _returnvalue_2)
  (`|ExecutionSequence`
    (:`then_0`
      ;[0.1551 0.2604 0.1524] RoadSign
      (bind _returnvalue_3 (`AddComponent|NODE_AddStaticMeshComponent-0` :`RelativeTransform` (`KismetMathLibrary.MakeTransform` (`KismetMathLibrary.MakeVector` 0.0 (`local.SignYLocation`)) (`KismetMathLibrary.MakeRotator` 0.0) (`KismetMathLibrary.MakeVector` (.x (.scale _signtransform)) 1.0 (.z (.scale _signtransform))))))
      (set `local.SignMeshComponent` _returnvalue_3)
      (`SceneComponent.K2_AttachToComponent` (`local.SignMeshComponent`) (`local.NULLParent`) "None" "KeepRelative" "KeepRelative" "KeepWorld" true)
      (`StaticMeshComponent.SetStaticMesh` (`local.SignMeshComponent`) (`local.SignMesh`))
      (bind _material (`self.CreateDynamicMetalMaterial` (`self.SignMetalMaterial`) (`local.SignMesh`)))
      (set `local.SignMetalMaterialInstance` _material)
      (`PrimitiveComponent.SetMaterialByName` (`local.SignMeshComponent`) "metal" _material)
      (bind _material_2 (`self.CreateDynamicSignMaterial` (`local.SignTexture`) (`local.isIridescent`) (`local.SignMesh`)))
      (bind _output_get (set `local.signMaterial` _material_2))
      (`PrimitiveComponent.SetMaterialByName` (`local.SignMeshComponent`) "sign" _output_get))
    (:`then_1`
      ;[0.08854 0.08854 0.08854] Attaches
      (for _index (range 1 5)
        (set `local.RailIndex` _index)
        (`/Engine/EditorBlueprintResources/StandardMacros.IsValid` (`StaticMesh.FindSocket` (`local.SignMesh`) (`KismetStringLibrary.Conv_StringToName` (`KismetStringLibrary.Concat_StrStr` "rail" (`KismetStringLibrary.Conv_IntToString` (`local.RailIndex`)))))
          (:`Is Valid`
            (if (`|EnumInequality` (`self.Pole Shape`) "NewEnumerator0")
              (bind _returnvalue_4 (`AddComponent|NODE_AddStaticMeshComponent-1` :`RelativeTransform` (`KismetMathLibrary.MakeTransform` (`KismetMathLibrary.MakeVector` (`local.PoleLocationX`) 0.0 (+ (* _relativelocation_z_3 (.z (.scale _signtransform_3))) (.z (.location _signtransform_3)))) (`KismetMathLibrary.MakeRotator` 0.0 0.0 (.yaw (.rotation _signtransform_3))))))
              (set `local.AttachMeshComponent` _returnvalue_4)
              (else
                (bind _returnvalue_5 (`AddComponent|NODE_AddStaticMeshComponent-2` :`RelativeTransform` (`KismetMathLibrary.MakeTransform` (`KismetMathLibrary.MakeVector` (.x (.location _signtransform_3)) 0.0 (+ (.z (.location _signtransform_3)) (* _relativelocation_z_3 (.z (.scale _signtransform_3))))) (`KismetMathLibrary.MakeRotator` 0.0 0.0 (.yaw (.rotation _signtransform_3))))))
                (set `local.AttachMeshComponent` _returnvalue_5)))
            (`SceneComponent.K2_AttachToComponent` (`local.AttachMeshComponent`) (`local.NULLParent`) "None" "KeepWorld" "KeepRelative" "KeepWorld" true)
            (bind _material_3 (`self.CreateDynamicMetalMaterial` (`self.AttachMaterial`) (`local.AttachMesh`)))
            (`MaterialInstanceDynamic.SetScalarParameterValue` _material_3 "DirtMap Offset" (`KismetMathLibrary.RandomFloat`))
            (`PrimitiveComponent.SetMaterial` (`local.AttachMeshComponent`) 0 _material_3)
            (`StaticMeshComponent.SetStaticMesh` (`local.AttachMeshComponent`) (`local.AttachMesh`)))
          (:`Is Not Valid`
            (break)))))
    (:`then_2`
      ;[1 1 1] Rail
      (`local.AttachMeshComponent`
        (:`then`
          (for _index_2 (range 1 5)
            (set `local.RailIndex` _index_2)
            (bind _returnvalue_6 (`StaticMesh.FindSocket` (`local.SignMesh`) (`KismetStringLibrary.Conv_StringToName` (`KismetStringLibrary.Concat_StrStr` "rail" (`KismetStringLibrary.Conv_IntToString` _index_2)))))
            (`/Engine/EditorBlueprintResources/StandardMacros.IsValid` _returnvalue_6
              (:`Is Valid`
                (bind (_relativelocation_x_9 _relativelocation_y_9 _relativelocation_z_4) (`KismetMathLibrary.BreakVector` (`StaticMeshSocket.RelativeLocation` _returnvalue_6)))
                (bind _relativescale_x (`KismetMathLibrary.BreakVector` (`StaticMeshSocket.RelativeScale` _returnvalue_6)))
                (bind _returnvalue_7 (`AddComponent|NODE_AddStaticMeshComponent-3` :`RelativeTransform` (`KismetMathLibrary.MakeTransform` (`KismetMathLibrary.MakeVector` (- (.x (.location (`local.SignTransform`))) _relativelocation_x_2) (- _relativelocation_y_7 _relativelocation_y_4) (- (* (.z (.scale _signtransform_2)) _relativelocation_z_4) _relativelocation_z_2)) (`KismetMathLibrary.MakeRotator` 0.0) (`KismetMathLibrary.MakeVector` (* _relativescale_x (.x (.scale _signtransform_2))) 1.0 1.0))))
                (set `local.RailMeshComponent` _returnvalue_7)
                (`SceneComponent.K2_AttachToComponent` _returnvalue_7 (`local.AttachMeshComponent`) (`KismetStringLibrary.Conv_StringToName` (`KismetStringLibrary.Concat_StrStr` "rail" (`KismetStringLibrary.Conv_IntToString` (`local.RailIndex`)))) "KeepRelative" "KeepRelative" "KeepWorld" true)
                (`StaticMeshComponent.SetStaticMesh` _returnvalue_7 (`/Game/RoadsignBP/Essentials/BP/BP_DA_Roadsign_Style.RailMesh` (`self.Style`)))
                (bind _material_4 (`self.CreateDynamicMetalMaterial` (`self.SignMetalMaterial`) (`/Game/RoadsignBP/Essentials/BP/BP_DA_Roadsign_Style.RailMesh` (`self.Style`))))
                (`MaterialInstanceDynamic.SetScalarParameterValue` _material_4 "DirtMap Offset" (`KismetMathLibrary.RandomFloat`))
                (`PrimitiveComponent.SetMaterial` _returnvalue_7 0 _material_4))
              (:`Is Not Valid`
                (break)))))
        (:`else`)))
    (:`then_3`
      ;[0.1775 0.1372 0.1979] Custom Rectangle
      (if (select `byte` (`local.SignShape`) :`0` false :`1` false :`2` false :`3` false :`4` false :`5` false :`6` false :`7` false :`8` false)
        (`MaterialInstanceDynamic.SetScalarParameterValue` (`local.signMaterial`) "UseCornerMask" (`KismetMathLibrary.Conv_BoolToDouble` (`/Game/RoadsignBP/Essentials/BP/BP_DA_Roadsign_Style.isRoundCorner` (`self.Style`))))
        (`MaterialInstanceDynamic.SetScalarParameterValue` (`local.SignMetalMaterialInstance`) "UseCornerMask" (`KismetMathLibrary.Conv_BoolToDouble` (`/Game/RoadsignBP/Essentials/BP/BP_DA_Roadsign_Style.isRoundCorner` (`self.Style`))))
        (`self.CreateCustomRectangle` (`local.SignMeshComponent`) (`local.SignMetalMaterialInstance`) (`local.signMaterial`) (`local.SignTransform`) (`self.Style`))))
    (:`then_4`
      (if (select `byte` (`local.SignShape`) :`0` false :`1` false :`2` false :`3` false :`4` false :`5` false :`6` false :`7` false :`8` false)
        (`self.CreateArrow` (`local.SignMeshComponent`) (`local.SignMetalMaterialInstance`) (`local.signMaterial`) (`local.SignTransform`) (`local.SignShape`) (`self.Style`))))
    (:`then_5`
      (`local.RailMeshComponent`
        (:`then`
          _)
        (:`else`
          (`KismetSystemLibrary.PrintString` (`KismetStringLibrary.Concat_StrStr` (`KismetSystemLibrary.GetDisplayName` self) " : Bad Roadsign Position") true true (struct :`R` 1.0 :`A` 1.0))))
      (`SceneComponent.K2_AttachToComponent` (`local.SignMeshComponent`) (select `bool` (`KismetSystemLibrary.IsValid` _railmeshcomponent) :`true` _railmeshcomponent :!type "SceneComponent Object Reference") "None" "KeepRelative" "KeepRelative" "KeepWorld" true)
      (`SceneComponent.K2_SetRelativeLocation` (`local.SignMeshComponent`) (`KismetMathLibrary.MakeVector` 0.0 0.0 (* _relativelocation_z -1.0)) false false))
    (:`then_6`
      (`|ExecutionSequence`
        (:`then_0`
          (for _array_element (`local.TextElements`)
            (`self.AddTextElement` _array_element (`local.SignMeshComponent`) (`local.isIridescent`) (`local.SignTransform`) (`self.Text Font`))))
        (:`then_1`
          (for _array_element_2 (`local.PictoElements`)
            (`self.AddPictoElement` _array_element_2 (`local.SignMeshComponent`) (`local.isIridescent`) (`local.SignTransform`))))))))

(fn `DefinePoleShape`
  (bind _parent (`self.Parent`))
  (`/Engine/EditorBlueprintResources/StandardMacros.IsValid` _parent
    (:`Is Valid`
      (bind _asbp_roadsign_1pole (cast `/Game/RoadsignBP/Blueprints/Method2/BP_Roadsign_1Pole` _parent)
        (:`then`
          (set `self.Pole Shape` (`/Game/RoadsignBP/Blueprints/Method2/BP_Roadsign_1Pole.PoleShape` _asbp_roadsign_1pole)))
        (:`CastFailed`
          (set `self.Pole Shape` (`self.Pole Shape`)))))))

(fn `DetachFromParent`
  (set `self.Parent` null)
  (`self.K2_DetachFromActor` "KeepWorld" "KeepWorld" "KeepWorld"))

(fn `Place to parent position`
  (bind _parent (`self.Parent`))
  (`self.Parent`
    (:`then`
      (`self.K2_SetActorLocationAndRotation` (`self.K2_GetActorLocation` _parent) (`self.K2_GetActorRotation` _parent)))
    (:`else`)))

(fn `SetBillboard`
  (bind _billboard (`self.Billboard`))
  (`self.Style`
    (:`then`
      (`SceneComponent.SetVisibility` _billboard false false))
    (:`else`
      (`SceneComponent.SetVisibility` _billboard true false))))

(fn `SetParent`
  (`/Engine/EditorBlueprintResources/StandardMacros.IsValid` (`self.Parent`)
    (:`Is Valid`
      (`self.K2_AttachToActor` (`self.Parent`) "None" "SnapToTarget" "SnapToTarget" "SnapToTarget"))
    (:`Is Not Valid`
      (`self.K2_DetachFromActor` "KeepWorld" "KeepWorld" "KeepWorld")
      (set `self.Parent` null))))

(fn `UserConstructionScript`
  (`parent.UserConstructionScript`)
  (`self.SetBillboard`)
  (`self.DefinePoleShape`)
  (`self.SetParent`)
  (`self.CreateRoadsign`))