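; Construction-script Blueprint for a single road sign pole, built from a selectable profile shape (round, square, rectangle or H).
; It adds the matching pole mesh stretched vertically by PoleHeight, plus a matching cap mesh offset by that height.
; The pole gets a dynamic metal material with a random dirt map offset to vary its look.
; When no shape is selected, only the billboard is made visible.
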(fn `CreatePole`
  (if (`|EnumInequality` (`self.PoleShape`) "NewEnumerator0")
    (bind _returnvalue (`AddComponent|NODE_AddStaticMeshComponent-0` :`RelativeTransform` (`KismetMathLibrary.MakeTransform` (0.0 0.0 0.0) (struct) (`KismetMathLibrary.MakeVector` 1.0 1.0 (`self.PoleHeight`))))) ; pole
    (`StaticMeshComponent.SetStaticMesh` _returnvalue (select `/Game/RoadsignBP/Essentials/Enums/Enum_PoleShape` (`self.PoleShape`) :`NewEnumerator1` "/Game/RoadsignBP/Essentials/StaticMesh/Pole/SM_roadsign_pole_round_60mm.SM_roadsign_pole_round_60mm" :`NewEnumerator2` "/Game/RoadsignBP/Essentials/StaticMesh/Pole/SM_roadsign_pole_round_76mm.SM_roadsign_pole_round_76mm" :`NewEnumerator3` "/Game/RoadsignBP/Essentials/StaticMesh/Pole/SM_roadsign_pole_square_40x40.SM_roadsign_pole_square_40x40" :`NewEnumerator4` "/Game/RoadsignBP/Essentials/StaticMesh/Pole/SM_roadsign_pole_square_80x80.SM_roadsign_pole_square_80x80" :`NewEnumerator5` "/Game/RoadsignBP/Essentials/StaticMesh/Pole/SM_roadsign_pole_rectangle_40x80.SM_roadsign_pole_rectangle_40x80" :`NewEnumerator6` "/Game/RoadsignBP/Essentials/StaticMesh/Pole/SM_roadsign_pole_H_100mm.SM_roadsign_pole_H_100mm" :!type "StaticMesh Object Reference"))
    (bind _material (`self.CreateDynamicMetalMaterial` (`self.PoleMaterial`)))
    (`MaterialInstanceDynamic.SetScalarParameterValue` _material "DirtMap Offset" (`KismetMathLibrary.RandomFloat`))
    (`PrimitiveComponent.SetMaterial` _returnvalue 0 _material)
    (bind _returnvalue_2 (`AddComponent|NODE_AddStaticMeshComponent-1` :`RelativeTransform` (`KismetMathLibrary.MakeTransform` (`KismetMathLibrary.MakeVector` 0.0 0.0 (`self.PoleHeight`))))) ; pole cap
    (`StaticMeshComponent.SetStaticMesh` _returnvalue_2 (select `/Game/RoadsignBP/Essentials/Enums/Enum_PoleShape` (`self.PoleShape`) :`NewEnumerator1` "/Game/RoadsignBP/Essentials/StaticMesh/Pole/SM_roadsign_pole_round_60mm_cap.SM_roadsign_pole_round_60mm_cap" :`NewEnumerator2` "/Game/RoadsignBP/Essentials/StaticMesh/Pole/SM_roadsign_pole_round_76mm_cap.SM_roadsign_pole_round_76mm_cap" :`NewEnumerator3` "/Game/RoadsignBP/Essentials/StaticMesh/Pole/SM_roadsign_pole_square_40x40_cap.SM_roadsign_pole_square_40x40_cap" :`NewEnumerator4` "/Game/RoadsignBP/Essentials/StaticMesh/Pole/SM_roadsign_pole_square_80x80_cap.SM_roadsign_pole_square_80x80_cap" :`NewEnumerator5` "/Game/RoadsignBP/Essentials/StaticMesh/Pole/SM_roadsign_pole_rectangle_40x80_cap.SM_roadsign_pole_rectangle_40x80_cap" :`NewEnumerator6` "/Game/RoadsignBP/Essentials/StaticMesh/Pole/SM_roadsign_pole_H_100mm_cap.SM_roadsign_pole_H_100mm_cap" :!type "StaticMesh Object Reference"))))

(fn `SetBillboard`
  (bind _billboard (`self.Billboard`))
  (if (`|EnumEquality` (`self.PoleShape`) "NewEnumerator0")
    (`SceneComponent.SetVisibility` _billboard true false)
    (else
      (`SceneComponent.SetVisibility` _billboard false false))))

(fn `UserConstructionScript`
  (`parent.UserConstructionScript`)
  (`self.SetBillboard`)
  (`self.CreatePole`))