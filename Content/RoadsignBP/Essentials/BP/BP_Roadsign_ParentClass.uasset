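; BP_Roadsign_ParentClass is a road sign base Blueprint providing helper functions that assemble signs from components, with empty event and construction graphs.
; Material helpers create dynamic metal and sign instances sharing dirt settings, carrying over the mesh's normal map.
; Pictogram and text helpers attach planes and text renders to the sign face, layered by Z-order offsets.
; Arrow and rectangle helpers fit style-specific end, side and corner meshes to panel bounds, handling mirrored scale.
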(fn `AddPictoElement`
  (params (PictoElement :type "/Game/RoadsignBP/Essentials/Structures/S_Roadsigns_Picto Structure") (SignMeshComponent :type "StaticMeshComponent Object Reference") (isIridescent :type Boolean) (SignTransform :type "Transform Structure"))
  (locals (PictoTexture :type "Texture2D Object Reference") (ColorOverride :type "LinearColor Structure") (PictoPosition :type "Vector2D Structure") (PictoScale :type "Vector2D Structure") (FitSize :type Boolean) (PictoZOrder :type Integer))
  (bind (_pictotexture _coloroverride _position _scale _fitsize _zorder) (break `/Game/RoadsignBP/Essentials/Structures/S_Roadsigns_Picto` PictoElement))
  (bind _pictotexture_2 (`local.PictoTexture`))
  (bind (_x _y) (`KismetMathLibrary.BreakVector2D` (`local.PictoPosition`)))
  (bind (_x_2 _y_2) (`KismetMathLibrary.BreakVector2D` (`local.PictoScale`)))
  (bind _returnvalue (`StaticMesh.GetBoundingBox` (`StaticMeshComponent.StaticMesh` (`local.SignMeshComponent`))))
  (bind _returnvalue_2 (* _y_2 0.15))
  (set `local.PictoTexture` _pictotexture)
  (set `local.ColorOverride` _coloroverride)
  (set `local.PictoPosition` _position)
  (set `local.PictoScale` _scale)
  (set `local.FitSize` _fitsize)
  (set `local.PictoZOrder` _zorder)
  (`/Engine/EditorBlueprintResources/StandardMacros.IsValid` (`local.PictoTexture`)
    (:`Is Valid`
      (bind _returnvalue_3 (`AddComponent|NODE_AddStaticMeshComponent-1` :`RelativeTransform` (`KismetMathLibrary.MakeTransform` (`KismetMathLibrary.MakeVector` (/ (+ (.x (`.Max` (break `Box` _returnvalue))) (.x (break `Box` _returnvalue))) 2.0) (.y (`.Max` (`StaticMeshComponent.GetLocalBounds` (`local.SignMeshComponent`))))) (struct :`Pitch` 180.0 :`Yaw` 180.0 :`Roll` -90.0) (select `bool` (`local.FitSize`) :`false` (`KismetMathLibrary.MakeVector` (* (* (/ (`Texture2D.Blueprint_GetSizeX` _pictotexture_2) (`Texture2D.Blueprint_GetSizeY` _pictotexture_2)) 0.15) _x_2) _returnvalue_2 _returnvalue_2) :`true` (`KismetMathLibrary.MakeVector` (.x (* (/ (`.BoxExtent` (`KismetSystemLibrary.GetComponentBounds` (`local.SignMeshComponent`))) 100) 2)) (.z (* (/ (`.BoxExtent` (`KismetSystemLibrary.GetComponentBounds` (`local.SignMeshComponent`))) 100) 2)) (.y (* (/ (`.BoxExtent` (`KismetSystemLibrary.GetComponentBounds` (`local.SignMeshComponent`))) 100) 2)))))))
      (`SceneComponent.K2_AttachToComponent` _returnvalue_3 (`local.SignMeshComponent`) "None" "KeepRelative" "KeepRelative" "KeepWorld" true)
      (`StaticMeshComponent.SetStaticMesh` _returnvalue_3 "/Engine/BasicShapes/Plane.Plane")
      (`PrimitiveComponent.SetCollisionEnabled` _returnvalue_3 "NoCollision")
      (`PrimitiveComponent.SetCastShadow` _returnvalue_3 false)
      (`SceneComponent.K2_AddRelativeLocation` _returnvalue_3 (`KismetMathLibrary.MakeVector` 0.0 (+ 0.025 (/ (`KismetMathLibrary.Conv_IntToDouble` (`local.PictoZOrder`)) 1000.0))) false false)
      (`SceneComponent.K2_AddRelativeLocation` _returnvalue_3 (`KismetMathLibrary.MakeVector` _x 0.0 _y) false false)
      (bind _returnvalue_4 (`PrimitiveComponent.CreateDynamicMaterialInstance` _returnvalue_3 0 "/Game/RoadsignBP/Essentials/Materials/Parents/InstanceParents/MI_RoadSign_Pictogram.MI_RoadSign_Pictogram" "None"))
      (`MaterialInstanceDynamic.SetTextureParameterValue` _returnvalue_4 "Sign" (`local.PictoTexture`))
      (`MaterialInstanceDynamic.SetScalarParameterValue` _returnvalue_4 "OpacityMask" 1.0)
      (`MaterialInstanceDynamic.SetScalarParameterValue` _returnvalue_4 "Grunge Amount" (`self.DirtAmount`))
      (`MaterialInstanceDynamic.SetScalarParameterValue` _returnvalue_4 "Iridescence" (`KismetMathLibrary.Conv_BoolToDouble` (`local.isIridescent`)))
      (`MaterialInstanceDynamic.SetScalarParameterValue` _returnvalue_4 "DirtMap Size" (`self.DirtMapSize`))
      (`MaterialInstanceDynamic.SetTextureParameterValue` _returnvalue_4 "Dirt Map" (`self.DirtMap`))
      (`MaterialInstanceDynamic.SetVectorParameterValue` _returnvalue_4 "Color Override" (`local.ColorOverride`)))))

(fn `AddTextElement`
  (params (TextElement :type "/Game/RoadsignBP/Essentials/Structures/S_Roadsigns_TextParameters Structure") (SignMeshComponent :type "StaticMeshComponent Object Reference") (isIridescent :type Boolean) (SignTransform :type "Transform Structure") (MainTextFont :type "Font Object Reference"))
  (locals (TextHorizontalAlignment :type "/Game/RoadsignBP/Essentials/Enums/Enum_TextAlignment Enum") (Text :type Text) (OverrideFont :type "Font Object Reference") (FontColor :type "LinearColor Structure") (TextSize :type "Float (double-precision)" :default 16.0) (TextPosition :type "Vector2D Structure") (TextZOrder :type Integer) (TextComponent :type "TextRenderComponent Object Reference") (TextBackgroundMesh :type "StaticMesh Object Reference" :default "/Script/Engine.StaticMesh'/Engine/BasicShapes/Plane.Plane'") (TextBackgroundComponent :type "StaticMeshComponent Object Reference") (TextBackgroundColor :type "LinearColor Structure"))
  (bind (_text _overridefont _textcolor _backgroundcolor _size _horizontalalignment _adjustposition _zorder) (break `/Game/RoadsignBP/Essentials/Structures/S_Roadsigns_TextParameters` TextElement))
  (bind _overridefont_2 (`local.OverrideFont`))
  (bind _signmeshcomponent (`local.SignMeshComponent`))
  (bind (_x _y) (`KismetMathLibrary.BreakVector2D` (`local.TextPosition`)))
  (bind _returnvalue (`StaticMesh.GetBoundingBox` (`local.TextBackgroundMesh`)))
  (bind (_returnvalue_x _returnvalue_y _returnvalue_z) (`KismetMathLibrary.BreakVector` (`TextRenderComponent.GetTextLocalSize` (`local.TextComponent`))))
  (bind (_min _max) (`StaticMeshComponent.GetLocalBounds` _signmeshcomponent))
  (bind _returnvalue_2 (`KismetMathLibrary.SignOfFloat` (.x (.scale (`local.SignTransform`)))))
  (bind _returnvalue_3 (`StaticMesh.GetBoundingBox` (`StaticMeshComponent.StaticMesh` _signmeshcomponent)))
  (bind _returnvalue_4 (* _returnvalue_2 6.0))
  (set `local.Text` _text)
  (set `local.OverrideFont` _overridefont)
  (set `local.FontColor` _textcolor)
  (set `local.TextBackgroundColor` _backgroundcolor)
  (set `local.TextSize` _size)
  (set `local.TextHorizontalAlignment` _horizontalalignment)
  (set `local.TextPosition` _adjustposition)
  (set `local.TextZOrder` _zorder)
  (`|ExecutionSequence`
    (:`then_0`
      ;[1 1 1] Text
      (if (not (`KismetTextLibrary.TextIsEmpty` (`local.Text`)))
        (bind _returnvalue_5 (`AddComponent|NODE_AddTextRenderComponent-0` :`RelativeTransform` (`KismetMathLibrary.MakeTransform` (`KismetMathLibrary.MakeVector` (select `/Game/RoadsignBP/Essentials/Enums/Enum_TextAlignment` (`local.TextHorizontalAlignment`) :`NewEnumerator0` (+ (* (.x _min) _returnvalue_2) _returnvalue_4) :`NewEnumerator1` (`KismetMathLibrary.Abs` (/ (+ (.x (`.Max` (break `Box` _returnvalue_3))) (.x (break `Box` _returnvalue_3))) 2.0)) :`NewEnumerator2` (- (* (.x _max) _returnvalue_2) _returnvalue_4)) (.y (`.Max` (`StaticMeshComponent.GetLocalBounds` (`local.SignMeshComponent`))))) (`KismetMathLibrary.MakeRotator` 0.0 0.0 (* 90.0 _returnvalue_2)) (1.0 1.0 1.0))))
        (set `local.TextComponent` _returnvalue_5)
        (`SceneComponent.K2_AttachToComponent` (`local.TextComponent`) (`local.SignMeshComponent`) "None" "KeepRelative" "KeepRelative" "KeepWorld" true)
        (`SceneComponent.K2_AddRelativeLocation` (`local.TextComponent`) (`KismetMathLibrary.MakeVector` 0.0 (+ 0.025 (/ (`KismetMathLibrary.Conv_IntToDouble` (`local.TextZOrder`)) 1000.0))) false false)
        (`SceneComponent.K2_AddRelativeLocation` (`local.TextComponent`) (`KismetMathLibrary.MakeVector` (* _x (`KismetMathLibrary.SignOfFloat` (.x (.scale (`local.SignTransform`))))) 0.0 _y) false false)
        (`TextRenderComponent.K2_SetText` (`local.TextComponent`) (`local.Text`))
        (`TextRenderComponent.SetFont` (`local.TextComponent`) (select `bool` (`KismetSystemLibrary.IsValid` _overridefont_2) :`false` (`local.MainTextFont`) :`true` _overridefont_2))
        (`TextRenderComponent.SetTextRenderColor` (`local.TextComponent`) (`KismetMathLibrary.Conv_LinearColorToColor` (`local.FontColor`) false))
        (`TextRenderComponent.SetWorldSize` (`local.TextComponent`) (`local.TextSize`))
        (`TextRenderComponent.SetHorizontalAlignment` (`local.TextComponent`) (select `byte` (`local.TextHorizontalAlignment`) :`0` "EHTA_Left" :`1` "EHTA_Center" :`2` "EHTA_Right" :!type "EHorizTextAligment Enum"))
        (bind _returnvalue_6 (`PrimitiveComponent.CreateDynamicMaterialInstance` (`local.TextComponent`) 0 "/Game/RoadsignBP/Essentials/Materials/Parents/MI_RoadSign_Font.MI_RoadSign_Font" "None"))
        (`MaterialInstanceDynamic.SetScalarParameterValue` _returnvalue_6 "Grunge Amount" (`self.DirtAmount`))
        (`MaterialInstanceDynamic.SetScalarParameterValue` _returnvalue_6 "Iridescence" (`KismetMathLibrary.Conv_BoolToDouble` (`local.isIridescent`)))
        (`MaterialInstanceDynamic.SetScalarParameterValue` _returnvalue_6 "DirtMap Size" (`self.DirtMapSize`))
        (`MaterialInstanceDynamic.SetTextureParameterValue` _returnvalue_6 "Dirt Map" (`self.DirtMap`))))
    (:`then_1`
      ;[1 1 1] Text Background Color
      (if (> (`.A` (`KismetMathLibrary.BreakColor` (`local.TextBackgroundColor`))) 0.0)
        (bind _returnvalue_7 (`AddComponent|NODE_AddStaticMeshComponent-2` :`RelativeTransform` (`KismetMathLibrary.MakeTransform` (`KismetMathLibrary.MakeVector` -0.01 (select `/Game/RoadsignBP/Essentials/Enums/Enum_TextAlignment` (`local.TextHorizontalAlignment`) :`NewEnumerator0` (/ _returnvalue_y -2.0) :`NewEnumerator2` (/ _returnvalue_y 2.0))) (struct :`Yaw` 90.0 :`Roll` -90.0) (`KismetMathLibrary.MakeVector` (* _returnvalue_y (/ 1.0 (- (.x (`.Max` (break `Box` _returnvalue))) (.x (break `Box` _returnvalue))))) (* _returnvalue_z (/ 1.0 (- (.y (`.Max` (break `Box` _returnvalue))) (.y (break `Box` _returnvalue))))) 1.0))))
        (set `local.TextBackgroundComponent` _returnvalue_7)
        (`SceneComponent.K2_AttachToComponent` (`local.TextBackgroundComponent`) (`local.TextComponent`) "None" "KeepRelative" "KeepRelative" "KeepWorld" true)
        (`StaticMeshComponent.SetStaticMesh` (`local.TextBackgroundComponent`) (`local.TextBackgroundMesh`))
        (bind _returnvalue_8 (`PrimitiveComponent.CreateDynamicMaterialInstance` (`local.TextBackgroundComponent`) 0 "/Game/RoadsignBP/Essentials/Materials/Parents/M_Roadsign_Sign.M_Roadsign_Sign" "None"))
        (`MaterialInstanceDynamic.SetTextureParameterValue` _returnvalue_8 "Sign" "/Interchange/gltf/Textures/T_White_Linear.T_White_Linear")
        (`MaterialInstanceDynamic.SetVectorParameterValue` _returnvalue_8 "Color Override" (`local.TextBackgroundColor`))
        (`MaterialInstanceDynamic.SetScalarParameterValue` _returnvalue_8 "Grunge Amount" (`self.DirtAmount`))
        (`MaterialInstanceDynamic.SetScalarParameterValue` _returnvalue_8 "Iridescence" 0.0)
        (`MaterialInstanceDynamic.SetScalarParameterValue` _returnvalue_8 "DirtMap Size" (`self.DirtMapSize`))
        (`MaterialInstanceDynamic.SetTextureParameterValue` _returnvalue_8 "Dirt Map" (`self.DirtMap`))))))

(fn `CreateArrow`
  (params (SignMeshComponent :type "StaticMeshComponent Object Reference") (MetalMaterial :type "MaterialInstanceDynamic Object Reference") (SignMaterial :type "MaterialInstanceDynamic Object Reference") (SignTransform :type "Transform Structure") (SignShape :type "/Game/RoadsignBP/Essentials/Enums/Enum_Roadsigns_SignShape Enum" :default "NewEnumerator0") (`Roadsign Style` :type "/Game/RoadsignBP/Essentials/BP/BP_DA_Roadsign_Style Object Reference"))
  (locals (ArrowStartComponent :type "StaticMeshComponent Object Reference") (ArrowEndComponent :type "StaticMeshComponent Object Reference") (ArrowStartMesh :type "StaticMesh Object Reference") (ArrowEndMesh :type "StaticMesh Object Reference"))
  (bind _roadsign_style (`local.Roadsign Style`))
  (bind _signtransform (`local.SignTransform`))
  (bind _roadsign_style_2 (`local.Roadsign Style`))
  (bind _returnvalue (`KismetMathLibrary.SignOfFloat` (.x (.scale (`local.signTransform`)))))
  (bind _returnvalue_2 (select `/Game/RoadsignBP/Essentials/Enums/Enum_Roadsigns_SignShape` (`local.SignShape`) :`NewEnumerator6` (`/Game/RoadsignBP/Essentials/BP/BP_DA_Roadsign_Style.ArrowEnd_1Lign` _roadsign_style_2) :`NewEnumerator7` (`/Game/RoadsignBP/Essentials/BP/BP_DA_Roadsign_Style.ArrowEnd_2Ligns` _roadsign_style_2) :`NewEnumerator8` (`/Game/RoadsignBP/Essentials/BP/BP_DA_Roadsign_Style.ArrowEnd_3Ligns` _roadsign_style_2)))
  (bind _returnvalue_3 (select `/Game/RoadsignBP/Essentials/Enums/Enum_Roadsigns_SignShape` (`local.SignShape`) :`NewEnumerator6` (`/Game/RoadsignBP/Essentials/BP/BP_DA_Roadsign_Style.ArrowStart_1Lign` _roadsign_style) :`NewEnumerator7` (`/Game/RoadsignBP/Essentials/BP/BP_DA_Roadsign_Style.ArrowStart_2Ligns` _roadsign_style) :`NewEnumerator8` (`/Game/RoadsignBP/Essentials/BP/BP_DA_Roadsign_Style.ArrowStart_3Ligns` _roadsign_style)))
  (`/Engine/EditorBlueprintResources/StandardMacros.IsValid` _returnvalue_3
    (:`Is Valid`
      (set `local.ArrowStartMesh` _returnvalue_3)
      (`/Engine/EditorBlueprintResources/StandardMacros.IsValid` _returnvalue_2
        (:`Is Valid`
          (set `local.ArrowEndMesh` _returnvalue_2)
          (`|ExecutionSequence`
            (:`then_0`
              (bind _returnvalue_4 (`AddComponent|NODE_AddStaticMeshComponent-3` :`RelativeTransform` (`KismetMathLibrary.MakeTransform` (`KismetMathLibrary.MakeVector` (.x (`StaticMeshComponent.GetLocalBounds` (`local.SignMeshComponent`)))) (struct) (`KismetMathLibrary.MakeVector` _returnvalue 1.0 (.z (.scale _signtransform))))))
              (bind _output_get (set `local.ArrowStartComponent` _returnvalue_4))
              (`StaticMeshComponent.SetStaticMesh` _output_get (`local.ArrowStartMesh`))
              (`SceneComponent.K2_AttachToComponent` _output_get (`local.SignMeshComponent`) "None" "KeepRelative" "KeepRelative" "KeepWorld" true))
            (:`then_1`
              (bind _returnvalue_5 (`AddComponent|NODE_AddStaticMeshComponent-4` :`RelativeTransform` (`KismetMathLibrary.MakeTransform` (`KismetMathLibrary.MakeVector` (.x (`.Max` (`StaticMeshComponent.GetLocalBounds` (`local.SignMeshComponent`))))) (struct) (`KismetMathLibrary.MakeVector` _returnvalue 1.0 (.z (.scale _signtransform))))))
              (bind _output_get_2 (set `local.ArrowEndComponent` _returnvalue_5))
              (`StaticMeshComponent.SetStaticMesh` _output_get_2 (`local.ArrowEndMesh`))
              (`SceneComponent.K2_AttachToComponent` _output_get_2 (`local.SignMeshComponent`) "None" "KeepRelative" "KeepRelative" "KeepWorld" true))
            (:`then_2`
              (`PrimitiveComponent.SetMaterialByName` (`local.ArrowStartComponent`) "metal" (`local.MetalMaterial`))
              (`PrimitiveComponent.SetMaterialByName` (`local.ArrowEndComponent`) "metal" (`local.MetalMaterial`))
              (`PrimitiveComponent.SetMaterialByName` (`local.ArrowStartComponent`) "sign" (`local.SignMaterial`))
              (`PrimitiveComponent.SetMaterialByName` (`local.ArrowEndComponent`) "sign" (`local.SignMaterial`)))))))))

(fn `CreateCustomRectangle`
  (params (CenterSignMeshComponent :type "StaticMeshComponent Object Reference") (metalMaterial :type "MaterialInterface Object Reference") (signMaterial :type "MaterialInstanceDynamic Object Reference") (signTransform :type "Transform Structure") (RoadsignStyle :type "/Game/RoadsignBP/Essentials/BP/BP_DA_Roadsign_Style Object Reference"))
  (locals (topComponent :type "StaticMeshComponent Object Reference") (bottomComponent :type "StaticMeshComponent Object Reference") (leftComponent :type "StaticMeshComponent Object Reference") (rightComponent :type "StaticMeshComponent Object Reference") (topLeftComponent :type "StaticMeshComponent Object Reference") (topRightComponent :type "StaticMeshComponent Object Reference") (bottomLeftComponent :type "StaticMeshComponent Object Reference") (bottomRightComponent :type "StaticMeshComponent Object Reference"))
  (bind _signtransform (`local.signTransform`))
  (bind _signtransform_2 (`local.signTransform`))
  (bind _signtransform_3 (`local.signTransform`))
  (bind _signtransform_4 (`local.signTransform`))
  (bind _signtransform_5 (`local.signTransform`))
  (bind _signtransform_6 (`local.signTransform`))
  (bind _min (`StaticMeshComponent.GetLocalBounds` (`local.CenterSignMeshComponent`)))
  (bind (_min_2 _max) (`StaticMeshComponent.GetLocalBounds` (`local.CenterSignMeshComponent`)))
  (bind _returnvalue (`KismetMathLibrary.SignOfFloat` (.z (.scale _signtransform_3))))
  (bind _returnvalue_2 (`KismetMathLibrary.SignOfFloat` (.z (.scale _signtransform_4))))
  (bind (_min_3 _max_2) (`StaticMeshComponent.GetLocalBounds` (`local.CenterSignMeshComponent`)))
  (bind (_min_4 _max_3) (`StaticMeshComponent.GetLocalBounds` (`local.CenterSignMeshComponent`)))
  (bind _returnvalue_3 (`StaticMesh.GetBoundingBox` (`/Game/RoadsignBP/Essentials/BP/BP_DA_Roadsign_Style.Side` (`local.RoadsignStyle`))))
  (bind _returnvalue_4 (`StaticMesh.GetBoundingBox` (`/Game/RoadsignBP/Essentials/BP/BP_DA_Roadsign_Style.Side` (`local.RoadsignStyle`))))
  (bind (_relativelocation_x _relativelocation_y _relativelocation_z) (`KismetMathLibrary.BreakVector` (`StaticMeshSocket.RelativeLocation` (`StaticMesh.FindSocket` (`/Game/RoadsignBP/Essentials/BP/BP_DA_Roadsign_Style.Corner` (`local.RoadsignStyle`)) "panel"))))
  (bind _relativelocation_x_2 (`KismetMathLibrary.BreakVector` (`StaticMeshSocket.RelativeLocation` (`StaticMesh.FindSocket` (`/Game/RoadsignBP/Essentials/BP/BP_DA_Roadsign_Style.Corner` (`local.RoadsignStyle`)) "panel"))))
  (bind _returnvalue_5 (* (/ (- (* (.z (`.BoxExtent` (`KismetSystemLibrary.GetComponentBounds` (`local.CenterSignMeshComponent`)))) 2.0) (`KismetMathLibrary.Abs` (* _relativelocation_z 2.0))) (- (.x (`.Max` (break `Box` _returnvalue_3))) (.x (break `Box` _returnvalue_3)))) (`KismetMathLibrary.SignOfFloat` (.x (.scale _signtransform_3)))))
  (bind _returnvalue_6 (* (/ (- (* (.x (`.BoxExtent` (`KismetSystemLibrary.GetComponentBounds` (`local.CenterSignMeshComponent`)))) 2.0) (`KismetMathLibrary.Abs` (* _relativelocation_x_2 2.0))) (- (.x (`.Max` (break `Box` _returnvalue_4))) (.x (break `Box` _returnvalue_4)))) (`KismetMathLibrary.SignOfFloat` (.x (.scale _signtransform_4)))))
  (`|ExecutionSequence`
    (:`then_0`
      (`/Game/RoadsignBP/Essentials/BP/BP_DA_Roadsign_Style.Side` (`local.RoadsignStyle`)
        (:`then`
          (bind _returnvalue_7 (`AddComponent|NODE_AddStaticMeshComponent-5` :`RelativeTransform` (`KismetMathLibrary.MakeTransform` (`KismetMathLibrary.MakeVector` 0.0 0.0 (.z (`.Max` (`StaticMeshComponent.GetLocalBounds` (`local.CenterSignMeshComponent`))))) (struct) (`KismetMathLibrary.MakeVector` _returnvalue_6 1.0 _returnvalue_2)))) ; top-center
          (bind _output_get (set `local.topComponent` _returnvalue_7))
          (`StaticMeshComponent.SetStaticMesh` _output_get (`/Game/RoadsignBP/Essentials/BP/BP_DA_Roadsign_Style.Side` (`local.RoadsignStyle`)))
          (`SceneComponent.K2_AttachToComponent` _output_get (`local.CenterSignMeshComponent`) "None" "KeepRelative" "KeepRelative" "KeepWorld" true)
          (bind _returnvalue_8 (`AddComponent|NODE_AddStaticMeshComponent-6` :`RelativeTransform` (`KismetMathLibrary.MakeTransform` (`KismetMathLibrary.MakeVector` 0.0 0.0 (.z (`StaticMeshComponent.GetLocalBounds` (`local.CenterSignMeshComponent`)))) (struct :`Pitch` 180.0) (`KismetMathLibrary.MakeVector` _returnvalue_6 1.0 _returnvalue_2)))) ; bottom-center
          (bind _output_get_2 (set `local.bottomComponent` _returnvalue_8))
          (`StaticMeshComponent.SetStaticMesh` _output_get_2 (`/Game/RoadsignBP/Essentials/BP/BP_DA_Roadsign_Style.Side` (`local.RoadsignStyle`)))
          (`SceneComponent.K2_AttachToComponent` _output_get_2 (`local.CenterSignMeshComponent`) "None" "KeepRelative" "KeepRelative" "KeepWorld" true)
          (bind _returnvalue_9 (`AddComponent|NODE_AddStaticMeshComponent-7` :`RelativeTransform` (`KismetMathLibrary.MakeTransform` (`KismetMathLibrary.MakeVector` (.x (`StaticMeshComponent.GetLocalBounds` (`local.CenterSignMeshComponent`)))) (struct :`Pitch` 90.0) (`KismetMathLibrary.MakeVector` _returnvalue_5 1.0 _returnvalue)))) ; left
          (bind _output_get_3 (set `local.leftComponent` _returnvalue_9))
          (`StaticMeshComponent.SetStaticMesh` _output_get_3 (`/Game/RoadsignBP/Essentials/BP/BP_DA_Roadsign_Style.Side` (`local.RoadsignStyle`)))
          (`SceneComponent.K2_AttachToComponent` _output_get_3 (`local.CenterSignMeshComponent`) "None" "KeepRelative" "KeepRelative" "KeepWorld" true)
          (bind _returnvalue_10 (`AddComponent|NODE_AddStaticMeshComponent-8` :`RelativeTransform` (`KismetMathLibrary.MakeTransform` (`KismetMathLibrary.MakeVector` (.x (`.Max` (`StaticMeshComponent.GetLocalBounds` (`local.CenterSignMeshComponent`))))) (struct :`Pitch` -90.0) (`KismetMathLibrary.MakeVector` _returnvalue_5 1.0 _returnvalue)))) ; right
          (bind _output_get_4 (set `local.rightComponent` _returnvalue_10))
          (`StaticMeshComponent.SetStaticMesh` _output_get_4 (`/Game/RoadsignBP/Essentials/BP/BP_DA_Roadsign_Style.Side` (`local.RoadsignStyle`)))
          (`SceneComponent.K2_AttachToComponent` _output_get_4 (`local.CenterSignMeshComponent`) "right" "KeepRelative" "KeepRelative" "KeepWorld" true))
        (:`else`)))
    (:`then_1`
      (`/Game/RoadsignBP/Essentials/BP/BP_DA_Roadsign_Style.Corner` (`local.RoadsignStyle`)
        (:`then`
          (bind _returnvalue_11 (`AddComponent|NODE_AddStaticMeshComponent-9` :`RelativeTransform` (`KismetMathLibrary.MakeTransform` (`KismetMathLibrary.MakeVector` (.x _min_3) 0.0 (.z _max_2)) (struct) (`KismetMathLibrary.MakeVector` (`KismetMathLibrary.SignOfFloat` (.x (.scale _signtransform_2))) 1.0 (`KismetMathLibrary.SignOfFloat` (.z (.scale _signtransform_2))))))) ; topLeft
          (bind _output_get_5 (set `local.topLeftComponent` _returnvalue_11))
          (`StaticMeshComponent.SetStaticMesh` _output_get_5 (`/Game/RoadsignBP/Essentials/BP/BP_DA_Roadsign_Style.Corner` (`local.RoadsignStyle`)))
          (`SceneComponent.K2_AttachToComponent` _output_get_5 (`local.CenterSignMeshComponent`) "None" "KeepRelative" "KeepRelative" "KeepWorld" true)
          (bind _returnvalue_12 (`AddComponent|NODE_AddStaticMeshComponent-10` :`RelativeTransform` (`KismetMathLibrary.MakeTransform` (`KismetMathLibrary.MakeVector` (.x _max_3) 0.0 (.z _max_3)) (struct :`Pitch` -90.0) (`KismetMathLibrary.MakeVector` (`KismetMathLibrary.SignOfFloat` (.x (.scale _signtransform_5))) 1.0 (`KismetMathLibrary.SignOfFloat` (.z (.scale _signtransform_5))))))) ; topRight
          (bind _output_get_6 (set `local.topRightComponent` _returnvalue_12))
          (`StaticMeshComponent.SetStaticMesh` _output_get_6 (`/Game/RoadsignBP/Essentials/BP/BP_DA_Roadsign_Style.Corner` (`local.RoadsignStyle`)))
          (`SceneComponent.K2_AttachToComponent` _output_get_6 (`local.CenterSignMeshComponent`) "None" "KeepRelative" "KeepRelative" "KeepWorld" true)
          (bind _returnvalue_13 (`AddComponent|NODE_AddStaticMeshComponent-11` :`RelativeTransform` (`KismetMathLibrary.MakeTransform` (`KismetMathLibrary.MakeVector` (.x _min) 0.0 (.z _min)) (struct :`Pitch` 90.0) (`KismetMathLibrary.MakeVector` (`KismetMathLibrary.SignOfFloat` (.x (.scale _signtransform_6))) 1.0 (`KismetMathLibrary.SignOfFloat` (.z (.scale _signtransform_6))))))) ; bottomLeft
          (bind _output_get_7 (set `local.bottomLeftComponent` _returnvalue_13))
          (`StaticMeshComponent.SetStaticMesh` _output_get_7 (`/Game/RoadsignBP/Essentials/BP/BP_DA_Roadsign_Style.Corner` (`local.RoadsignStyle`)))
          (`SceneComponent.K2_AttachToComponent` _output_get_7 (`local.CenterSignMeshComponent`) "None" "KeepRelative" "KeepRelative" "KeepWorld" true)
          (bind _returnvalue_14 (`AddComponent|NODE_AddStaticMeshComponent-12` :`RelativeTransform` (`KismetMathLibrary.MakeTransform` (`KismetMathLibrary.MakeVector` (.x _max) 0.0 (.z _min_2)) (struct :`Pitch` 180.0) (`KismetMathLibrary.MakeVector` (`KismetMathLibrary.SignOfFloat` (.x (.scale _signtransform))) 1.0 (`KismetMathLibrary.SignOfFloat` (.z (.scale _signtransform))))))) ; bottomRight
          (bind _output_get_8 (set `local.bottomRightComponent` _returnvalue_14))
          (`StaticMeshComponent.SetStaticMesh` _output_get_8 (`/Game/RoadsignBP/Essentials/BP/BP_DA_Roadsign_Style.Corner` (`local.RoadsignStyle`)))
          (`SceneComponent.K2_AttachToComponent` _output_get_8 (`local.CenterSignMeshComponent`) "None" "KeepRelative" "KeepRelative" "KeepWorld" true)
          (`PrimitiveComponent.SetMaterialByName` (`local.topComponent`) "metal" (`local.metalMaterial`))
          (`PrimitiveComponent.SetMaterialByName` (`local.bottomComponent`) "metal" (`local.metalMaterial`))
          (`PrimitiveComponent.SetMaterialByName` (`local.leftComponent`) "metal" (`local.metalMaterial`))
          (`PrimitiveComponent.SetMaterialByName` (`local.rightComponent`) "metal" (`local.metalMaterial`))
          (`PrimitiveComponent.SetMaterialByName` (`local.bottomRightComponent`) "metal" (`local.metalMaterial`))
          (`PrimitiveComponent.SetMaterialByName` (`local.bottomLeftComponent`) "metal" (`local.metalMaterial`))
          (`PrimitiveComponent.SetMaterialByName` (`local.topRightComponent`) "metal" (`local.metalMaterial`))
          (`PrimitiveComponent.SetMaterialByName` (`local.topLeftComponent`) "metal" (`local.metalMaterial`)))
        (:`else`)))))

(fn `CreateDynamicMetalMaterial`
  (params (ParentMaterial :type "MaterialInterface Object Reference") (Mesh :type "StaticMesh Object Reference"))
  (returns (Material :type "MaterialInstanceDynamic Object Reference"))
  (bind _returnvalue (`KismetMaterialLibrary.CreateDynamicMaterialInstance` ParentMaterial))
  (`MaterialInstanceDynamic.SetScalarParameterValue` _returnvalue "Grunge Amount" (`self.DirtAmount`))
  (`MaterialInstanceDynamic.SetScalarParameterValue` _returnvalue "DirtMap Size" (`self.DirtMapSize`))
  (`MaterialInstanceDynamic.SetTextureParameterValue` _returnvalue "Dirt Map" (`self.DirtMap`))
  (`MaterialInstanceDynamic.SetTextureParameterValue` _returnvalue "Normal" (`self.GetNormalFromMesh` (`local.Mesh`)))
  (return _returnvalue))

(fn `CreateDynamicSignMaterial`
  (params (SignTexture :type "Texture2D Object Reference") (isIridescent :type Boolean) (SignMesh :type "StaticMesh Object Reference"))
  (returns (Material :type "MaterialInstanceDynamic Object Reference"))
  (bind _returnvalue (`StaticMesh.GetMaterial` SignMesh (`StaticMesh.GetMaterialIndex` SignMesh "sign")))
  (bind _returnvalue_2 (`MaterialInterface.GetBaseMaterial` _returnvalue))
  (bind _returnvalue_3 (`KismetMaterialLibrary.CreateDynamicMaterialInstance` (select `bool` (and (`KismetSystemLibrary.IsValid` _returnvalue) (== _returnvalue_2 "/Game/RoadsignBP/Essentials/Materials/Parents/M_Roadsign_Sign.M_Roadsign_Sign")) :`false` "/Game/RoadsignBP/Essentials/Materials/Parents/M_Roadsign_Sign.M_Roadsign_Sign" :`true` _returnvalue) "Sign"))
  (`MaterialInstanceDynamic.SetTextureParameterValue` _returnvalue_3 "Sign" (`local.SignTexture`))
  (`MaterialInstanceDynamic.SetScalarParameterValue` _returnvalue_3 "Grunge Amount" (`self.DirtAmount`))
  (`MaterialInstanceDynamic.SetScalarParameterValue` _returnvalue_3 "Iridescence" (`KismetMathLibrary.Conv_BoolToDouble` (`local.isIridescent`)))
  (`MaterialInstanceDynamic.SetScalarParameterValue` _returnvalue_3 "DirtMap Size" (`self.DirtMapSize`))
  (`MaterialInstanceDynamic.SetTextureParameterValue` _returnvalue_3 "Dirt Map" (`self.DirtMap`))
  (return _returnvalue_3))

(fn `GetNormalFromMesh`
  (params (Mesh :type "StaticMesh Object Reference"))
  (returns (Normal :type "Texture Object Reference"))
  (`/Engine/EditorBlueprintResources/StandardMacros.IsValid` Mesh
    (:`Is Valid`
      (bind _returnvalue (`KismetMaterialLibrary.CreateDynamicMaterialInstance` (`StaticMesh.GetMaterial` Mesh (`StaticMesh.GetMaterialIndex` Mesh "metal"))))
      (bind _returnvalue_2 (`MaterialInstanceDynamic.K2_GetTextureParameterValue` _returnvalue "Normal"))
      (return (select `bool` (== _returnvalue_2 null) :`false` _returnvalue_2)))))

(fn `UserConstructionScript`)