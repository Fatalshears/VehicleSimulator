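; RAM TRX four-wheeled vehicle Blueprint that adds steering assistance along GuidingPath splines on top of its parent's behavior.
; On BeginPlay and on a looping timer, it scans all GuidingPath actors and caches the one whose spline point is nearest the vehicle.
; Each Tick, when paths exist and ControlledSteer is zero, it feeds AutoSteer's result from that path and the vehicle's transform into the movement component's steering input.
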(event `self.ReceiveBeginPlay`
  (bind _returnvalue (`self.K2_GetActorLocation`))
  (`parent.ReceiveBeginPlay`)
  (`KismetSystemLibrary.K2_SetTimerDelegate` (delegate `FindNearestPath`) 5.0 true)
  (bind _outactors (`GameplayStatics.GetAllActorsOfClass` "/Game/MyContent/MyBlueprint/GuidingPath.GuidingPath_C" :!label _label))
  (set `self.NoGuiding` (`KismetArrayLibrary.Array_IsEmpty` _outactors))
  (for (_array_element _array_index) _outactors
    (if (== _array_index 0)
      (bind _returnvalue_2 (`SplineComponent.FindLocationClosestToWorldLocation` (`/Game/MyContent/MyBlueprint/GuidingPath.Spline` _array_element) _returnvalue "World"))
      (set `self.ClosestDistance` (`KismetMathLibrary.VSize` (- _returnvalue _returnvalue_2)))
      (else
        (bind _returnvalue_3 (`KismetMathLibrary.VSize` (- _returnvalue _returnvalue_2)))
        (if (< _returnvalue_3 (`self.ClosestDistance`))
          (set `self.GuidingPath_id` _array_index)
          (set `self.ClosestDistance` _returnvalue_3)))))
  (set `self.ClosetSpline` (`|GetArrayItem` _outactors (`self.GuidingPath_id`))))

(event `FindNearestPath`
  (goto _label))

(event `self.ReceiveTick`
  (params (DeltaSeconds :type "Float (single-precision)"))
  (`parent.ReceiveTick` DeltaSeconds)
  (if (`self.NoGuiding`)
    _
    (elif (== (`self.Controlled_Steer`) 0.0)
      (bind _steer (`/Game/MyContent/MyLib/BPL_Control_Object.Auto_Steer` (`self.ClosetSpline`) (`self.K2_GetActorLocation`) (`self.K2_GetActorRotation`)))
      (`ChaosVehicleMovementComponent.SetSteeringInput` (`self.VehicleMovementComponent`) _steer))))

(fn `UserConstructionScript`
  (`parent.UserConstructionScript`))