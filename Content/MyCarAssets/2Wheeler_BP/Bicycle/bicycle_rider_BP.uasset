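; Bicycle rider vehicle Blueprint that leans the bicycle and exposes riding data, built on a vehicle movement component.
; Each tick it smoothly rolls the bicycle by steering input scaled with speed and clamped, adding a fixed tilt when nearly stationary.
; Getter functions supply first-wheel angular velocity, raw steering input, and seat, handle, footrest and stop-foot locations relative to the rider mannequin.
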(event `self.ReceiveTick`
  (params (DeltaSeconds :type "Float (single-precision)"))
  (bind _bicycle (`self.bicycle`))
  (bind _vehiclemovementcomponent (`self.VehicleMovementComponent`))
  (bind _returnvalue (`KismetMathLibrary.VSize` (`self.GetVelocity` (`PawnMovementComponent.GetPawnOwner` _vehiclemovementcomponent))))
  ;[1 1 1] Motorbike lean when steering
  (`/Engine/EditorBlueprintResources/StandardMacros.IsValid` _bicycle
    (:`Is Valid`
      (bind _returnvalue_2 (`ChaosVehicleMovementComponent.GetSteeringInput` _vehiclemovementcomponent))
      (`SceneComponent.K2_SetRelativeRotation` _bicycle (`KismetMathLibrary.MakeRotator` (`self.LeanAngle`)) false false)
      (set `self.LeanAngle` (`KismetMathLibrary.Lerp` (`self.LeanAngle`) (+ (`KismetMathLibrary.FClamp` (* (* _returnvalue_2 40.0) (/ _returnvalue 1000.0)) -30.0 30.0) (`KismetMathLibrary.SelectFloat` 20.0 0.0 (and (< _returnvalue 20.0) (>= _returnvalue -20.0)))) 0.05)))))

(fn `GetAcceleration`
  (returns (Acceleration :type "Float (double-precision)"))
  (bind _aschaos_wheeled_vehicle_movement_component (cast `ChaosWheeledVehicleMovementComponent` (`self.VehicleMovementComponent`)))
  (return (`ChaosVehicleWheel.GetWheelAngularVelocity` (`|GetArrayItem` (`ChaosWheeledVehicleMovementComponent.Wheels` _aschaos_wheeled_vehicle_movement_component)))))

(fn `GetMotorBikePoints`
  (returns (Seat :type "Vector Structure") (LeftHandle :type "Vector Structure") (RightHandle :type "Vector Structure") (LeftFootRest :type "Vector Structure") (RightFootRest :type "Vector Structure") (RightFootStop :type "Vector Structure"))
  (bind _sk_mannequin (`self.SK_Mannequin`))
  (bind _returnvalue_location (`KismetMathLibrary.BreakTransform` (`KismetMathLibrary.MakeRelativeTransform` (`SceneComponent.K2_GetComponentToWorld` (`self.Seat`)) (`SceneComponent.K2_GetComponentToWorld` _sk_mannequin))))
  (bind _returnvalue_location_2 (`KismetMathLibrary.BreakTransform` (`KismetMathLibrary.MakeRelativeTransform` (`SceneComponent.K2_GetComponentToWorld` (`self.LeftHandle`)) (`SceneComponent.K2_GetComponentToWorld` _sk_mannequin))))
  (bind _returnvalue_location_3 (`KismetMathLibrary.BreakTransform` (`KismetMathLibrary.MakeRelativeTransform` (`SceneComponent.K2_GetComponentToWorld` (`self.RightHandle`)) (`SceneComponent.K2_GetComponentToWorld` _sk_mannequin))))
  (bind _returnvalue_location_4 (`KismetMathLibrary.BreakTransform` (`KismetMathLibrary.MakeRelativeTransform` (`SceneComponent.K2_GetComponentToWorld` (`self.LeftFootRest`)) (`SceneComponent.K2_GetComponentToWorld` _sk_mannequin))))
  (bind _returnvalue_location_5 (`KismetMathLibrary.BreakTransform` (`KismetMathLibrary.MakeRelativeTransform` (`SceneComponent.K2_GetComponentToWorld` (`self.RightFootStop`)) (`SceneComponent.K2_GetComponentToWorld` _sk_mannequin))))
  (bind _returnvalue_location_6 (`KismetMathLibrary.BreakTransform` (`KismetMathLibrary.MakeRelativeTransform` (`SceneComponent.K2_GetComponentToWorld` (`self.RightFootRest`)) (`SceneComponent.K2_GetComponentToWorld` _sk_mannequin))))
  (`/Engine/EditorBlueprintResources/StandardMacros.IsValid` _sk_mannequin
    (:`Is Valid`
      (return _returnvalue_location _returnvalue_location_2 _returnvalue_location_3 _returnvalue_location_4 _returnvalue_location_6 _returnvalue_location_5))))

(fn `GetTurnAngle`
  (returns (TurnAngle :type "Float (double-precision)"))
  (bind _returnvalue (`ChaosVehicleMovementComponent.GetSteeringInput` (`self.VehicleMovementComponent`)))
  (return _returnvalue))

(fn `UserConstructionScript`)