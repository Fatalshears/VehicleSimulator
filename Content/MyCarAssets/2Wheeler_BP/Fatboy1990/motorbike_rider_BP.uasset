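; Rideable motorbike vehicle Blueprint with a mannequin rider, spline-based steering assist and visual leaning.
; A looping timer caches the nearest GuidingPath, which feeds AutoSteer on Tick whenever ControlledSteer is zero.
; Tick also rolls the bike mesh by steering and speed, smoothed with a Lerp and tilted slightly when nearly stationary.
; Getters expose steering input and seat, handle and foot points in mannequin space, apparently for rider posing.
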(event `self.ReceiveBeginPlay`
  (bind _returnvalue (`self.K2_GetActorLocation`))
  (`KismetSystemLibrary.K2_SetTimerDelegate` (delegate `FindNearestPath`) 5.0 true)
  (bind _outactors (`GameplayStatics.GetAllActorsOfClass` "/Game/MyContent/MyBlueprint/GuidingPath.GuidingPath_C" :!label _label))
  (set `self.NoGuiding` (`KismetArrayLibrary.Array_IsEmpty` _outactors))
  (for (_array_element _array_index) _outactors
    (if (== _array_index 0)
      (bind _returnvalue_2 (`SplineComponent.FindLocationClosestToWorldLocation` (`/Game/MyContent/MyBlueprint/GuidingPath.Spline` _array_element) _returnvalue "World"))
      (set `self.ClosestDistance` (`KismetMathLibrary.VSize` (- _returnvalue _returnvalue_2)))
      (else
        (bind _returnvalue_3 (`KismetMathLibrary.VSize` (- _returnvalue _returnvalue_2)))
        (if (< _returnvalue_3 (`self.ClosestDistance`))
          (set `self.GuidingPath_id` _array_index)
          (set `self.ClosestDistance` _returnvalue_3)))))
  (set `self.ClosetSpline` (`|GetArrayItem` _outactors (`self.GuidingPath_id`))))

(event `FindNearestPath`
  (goto _label))

(event `self.ReceiveTick`
  (params (DeltaSeconds :type "Float (single-precision)"))
  (bind _vehiclemovementcomponent (`self.VehicleMovementComponent`))
  (bind _fatboy_motorbike (`self.fatboy_motorbike`))
  (bind _returnvalue (`KismetMathLibrary.VSize` (`self.GetVelocity` (`PawnMovementComponent.GetPawnOwner` _vehiclemovementcomponent))))
  ;[1 1 1] Motorbike lean when steering
  (`|ExecutionSequence`
    (:`then_0`
      (if (`self.NoGuiding`)
        _
        (elif (== (`self.Controlled_Steer`) 0.0)
          (bind _steer (`/Game/MyContent/MyLib/BPL_Control_Object.Auto_Steer` (`self.ClosetSpline`) (`self.K2_GetActorLocation`) (`self.K2_GetActorRotation`)))
          (`ChaosVehicleMovementComponent.SetSteeringInput` (`self.VehicleMovementComponent`) _steer))))
    (:`then_1`
      (`/Engine/EditorBlueprintResources/StandardMacros.IsValid` _fatboy_motorbike
        (:`Is Valid`
          (bind _returnvalue_2 (`ChaosVehicleMovementComponent.GetSteeringInput` _vehiclemovementcomponent))
          (`SceneComponent.K2_SetRelativeRotation` _fatboy_motorbike (`KismetMathLibrary.MakeRotator` (`self.LeanAngle`)) false false)
          (set `self.LeanAngle` (`KismetMathLibrary.Lerp` (`self.LeanAngle`) (+ (`KismetMathLibrary.FClamp` (* (* _returnvalue_2 40.0) (/ _returnvalue 1000.0)) -30.0 30.0) (`KismetMathLibrary.SelectFloat` 8.0 0.0 (and (< _returnvalue 20.0) (>= _returnvalue -20.0)))) 0.05)))))))

(fn `GetMotorBikePoints`
  (returns (Seat :type "Vector Structure") (LeftHandle :type "Vector Structure") (RightHandle :type "Vector Structure") (LeftFootRest :type "Vector Structure") (RightFootRest :type "Vector Structure") (RightFootStop :type "Vector Structure"))
  (bind _sk_mannequin (`self.SK_Mannequin`))
  (bind _returnvalue_location (`KismetMathLibrary.BreakTransform` (`KismetMathLibrary.MakeRelativeTransform` (`SceneComponent.K2_GetComponentToWorld` (`self.Seat`)) (`SceneComponent.K2_GetComponentToWorld` _sk_mannequin))))
  (bind _returnvalue_location_2 (`KismetMathLibrary.BreakTransform` (`KismetMathLibrary.MakeRelativeTransform` (`SceneComponent.K2_GetComponentToWorld` (`self.LeftHandle`)) (`SceneComponent.K2_GetComponentToWorld` _sk_mannequin))))
  (bind _returnvalue_location_3 (`KismetMathLibrary.BreakTransform` (`KismetMathLibrary.MakeRelativeTransform` (`SceneComponent.K2_GetComponentToWorld` (`self.RightHandle`)) (`SceneComponent.K2_GetComponentToWorld` _sk_mannequin))))
  (bind _returnvalue_location_4 (`KismetMathLibrary.BreakTransform` (`KismetMathLibrary.MakeRelativeTransform` (`SceneComponent.K2_GetComponentToWorld` (`self.LeftFootRest`)) (`SceneComponent.K2_GetComponentToWorld` _sk_mannequin))))
  (bind _returnvalue_location_5 (`KismetMathLibrary.BreakTransform` (`KismetMathLibrary.MakeRelativeTransform` (`SceneComponent.K2_GetComponentToWorld` (`self.RightFootStop`)) (`SceneComponent.K2_GetComponentToWorld` _sk_mannequin))))
  (bind _returnvalue_location_6 (`KismetMathLibrary.BreakTransform` (`KismetMathLibrary.MakeRelativeTransform` (`SceneComponent.K2_GetComponentToWorld` (`self.RightFootRest`)) (`SceneComponent.K2_GetComponentToWorld` _sk_mannequin))))
  (`/Engine/EditorBlueprintResources/StandardMacros.IsValid` _sk_mannequin
    (:`Is Valid`
      (return _returnvalue_location _returnvalue_location_2 _returnvalue_location_3 _returnvalue_location_4 _returnvalue_location_6 _returnvalue_location_5))))

(fn `GetTurnAngle`
  (returns (TurnAngle :type "Float (double-precision)"))
  (bind _returnvalue (`ChaosVehicleMovementComponent.GetSteeringInput` (`self.VehicleMovementComponent`)))
  (return _returnvalue))

(fn `UserConstructionScript`)